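; Map function actor that simulates a player in a mouse lane-defence game, automatically choosing and placing cards on the map grid.
; InitCardData keeps ground cards and starts a randomly delayed loop that repeats until game over.
; Each tick sorts cards by role, picks randomly within a role based on mice present, and scans role-specific rows or columns for a free cell.
; PlayCard places cards by issuing "/game play" text instructions rather than spawning them directly.
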(event `self.ReceiveDestroyed`
  ;[1 1 1] 被销毁
  (`KismetSystemLibrary.K2_ClearAndInvalidateTimerHandle` (`self.TimeHandle`)))

(event `self.Init Card Data`
  (params (Cards :type "Map of String to /Game/Resource/BP/Data/CardData/DialogueChar/PlayCardStruct Structure"))
  (set `self.CardsData` Cards)
  (`|ExecutionSequence`
    (:`then_0`
      ;[1 1 1] 初始化卡片分类
      (`self.CategoryCards` (`self.CardsData`)))
    (:`then_1`
      ;[1 1 1] 开始模拟操作
      (add `self.InitOperate` (delegate `Begin`))
      (`self.InitOperate`))))

(event `Begin`
  ;[1 1 1] 操作细节
  (bind _returnvalue (`KismetSystemLibrary.K2_SetTimerDelegate` (delegate `LoopBody`) (`KismetMathLibrary.RandomFloatInRange` 4.0 5.0)))
  (set `self.TimeHandle` _returnvalue))

(event `LoopBody`
  ;[1 1 1] 操作细节
  (if (`self.GetGameOver`)
    (`KismetSystemLibrary.K2_ClearAndInvalidateTimerHandle` (`self.TimeHandle`))
    (clear `self.InitOperate`)
    (else
      (`self.BeginOperate`)
      (`self.InitOperate`))))

(event `self.BeginOperate`
  (`self.InitPlayCardState`)
  (`self.Play Card to Ground` (`self.GroundData`)))

(fn `CategoryCards`
  (params (Cards :type "Map of String to /Game/Resource/BP/Data/CardData/DialogueChar/PlayCardStruct Structure"))
  (locals (CurData :type "/Game/Resource/BP/Data/CardData/DialogueChar/PlayCardStruct Structure") (CurCardName :type String))
  (bind (_curdata_grade _curdata_id _curdata_playtype) (break `/Game/Resource/BP/Data/CardData/DialogueChar/PlayCardStruct` (`local.CurData`)))
  (bind _keys (`BlueprintMapLibrary.Map_Keys` Cards))
  (for (_array_element _array_index) _keys
    (set `local.CurCardName` _array_element)
    (bind _values (`BlueprintMapLibrary.Map_Values` (`local.Cards`)))
    (set `local.CurData` (`|GetArrayItem` _values _array_index))
    (switch `/Game/Resource/BP/Data/CardData/DialogueChar/PlayCardPlayType` _curdata_playtype
      (:`NewEnumerator0`
        (`BlueprintMapLibrary.Map_Add` (`self.GroundData`) (`local.CurCardName`) (`local.CurData`))))))

(fn `CategroyCardsByGround`
  (params (Datas :type "Map of String to /Game/Resource/BP/Data/CardData/DialogueChar/PlayCardStruct Structure"))
  (returns (Spawn1 :type "Map of String to /Game/Resource/BP/Data/CardData/DialogueChar/PlayCardStruct Structure") (ATK_Line1 :type "Map of String to /Game/Resource/BP/Data/CardData/DialogueChar/PlayCardStruct Structure") (ATK_Proj1 :type "Map of String to /Game/Resource/BP/Data/CardData/DialogueChar/PlayCardStruct Structure") (Func_Bomb1 :type "Map of String to /Game/Resource/BP/Data/CardData/DialogueChar/PlayCardStruct Structure") (Func_PlayBomb1 :type "Map of String to /Game/Resource/BP/Data/CardData/DialogueChar/PlayCardStruct Structure") (Defence_Def1 :type "Map of String to /Game/Resource/BP/Data/CardData/DialogueChar/PlayCardStruct Structure") (Defence_Safe1 :type "Map of String to /Game/Resource/BP/Data/CardData/DialogueChar/PlayCardStruct Structure"))
  (locals (CurCardName :type String) (CurData :type "/Game/Resource/BP/Data/CardData/DialogueChar/PlayCardStruct Structure") (Spawn :type "Map of String to /Game/Resource/BP/Data/CardData/DialogueChar/PlayCardStruct Structure") (ATK_Line :type "Map of String to /Game/Resource/BP/Data/CardData/DialogueChar/PlayCardStruct Structure") (ATK_Proj :type "Map of String to /Game/Resource/BP/Data/CardData/DialogueChar/PlayCardStruct Structure") (Func_Bomb :type "Map of String to /Game/Resource/BP/Data/CardData/DialogueChar/PlayCardStruct Structure") (Func_PlayBomb :type "Map of String to /Game/Resource/BP/Data/CardData/DialogueChar/PlayCardStruct Structure") (Defence_Def :type "Map of String to /Game/Resource/BP/Data/CardData/DialogueChar/PlayCardStruct Structure") (Defence_Safe :type "Map of String to /Game/Resource/BP/Data/CardData/DialogueChar/PlayCardStruct Structure"))
  (bind _keys (`BlueprintMapLibrary.Map_Keys` Datas))
  (for (_array_element _array_index) _keys
    (set `local.CurCardName` _array_element)
    (bind _values (`BlueprintMapLibrary.Map_Values` Datas))
    (bind _output_get (set `local.CurData` (`|GetArrayItem` _values _array_index)))
    (switch `/Game/Resource/BP/Data/CardData/DialogueChar/PlayCardPlayCategory` (`.PlayCategroy_10_EFE9311B41F9C647B34931B7D08C4C3D` (break `/Game/Resource/BP/Data/CardData/DialogueChar/PlayCardStruct` _output_get))
      (:`NewEnumerator2`
        (`BlueprintMapLibrary.Map_Add` (`local.Spawn`) (`local.CurCardName`) (`local.CurData`)))
      (:`NewEnumerator0`
        (`BlueprintMapLibrary.Map_Add` (`local.ATK_Line`) (`local.CurCardName`) (`local.CurData`)))
      (:`NewEnumerator1`
        (`BlueprintMapLibrary.Map_Add` (`local.ATK_Proj`) (`local.CurCardName`) (`local.CurData`)))
      (:`NewEnumerator3`
        (`BlueprintMapLibrary.Map_Add` (`local.Func_Bomb`) (`local.CurCardName`) (`local.CurData`)))
      (:`NewEnumerator4`
        (`BlueprintMapLibrary.Map_Add` (`local.Func_PlayBomb`) (`local.CurCardName`) (`local.CurData`)))
      (:`NewEnumerator5`
        (`BlueprintMapLibrary.Map_Add` (`local.Defence_Def`) (`local.CurCardName`) (`local.CurData`)))
      (:`NewEnumerator6`
        (`BlueprintMapLibrary.Map_Add` (`local.Defence_Safe`) (`local.CurCardName`) (`local.CurData`)))))
  (return (`local.Spawn`) (`local.ATK_Line`) (`local.ATK_Proj`) (`local.Func_Bomb`) (`local.Func_PlayBomb`) (`local.Defence_Def`) (`local.Defence_Safe`)))

(fn `Check Def Meshe`
  (params (PlayType :type "/Game/Resource/BP/Data/CardData/DialogueChar/PlayCardPlayType Enum" :default "NewEnumerator0"))
  (locals (MesheComp :type "MesheControllComponent Object Reference") (RowAndCol :type "Line Structure" :default (struct)))
  (bind _playtargetline_row (break `Line` (`self.PlayTargetLine`)))
  (if (not (`self.bPlay`))
    (bind _returnvalue (`GameMapInstance.GetGameMapInstance`))
    (bind _returnvalue_2 (`GameMapInstance.GetMesheControllComponent` _returnvalue))
    (set `local.MesheComp` _returnvalue_2)
    (bind _returnvalue_3 (`MesheControllComponent.GetMapMeshRowAndCol` (`local.MesheComp`)))
    (set `local.RowAndCol` _returnvalue_3)
    (set `self.PlayTargetLine` (make `Line` -1 -1))
    (`|ExecutionSequence`
      (:`then_0`
        (switch `/Game/Resource/BP/Data/CardData/DialogueChar/PlayCardPlayType` PlayType
          (:`NewEnumerator0`
            (`self.CheckDef` (`local.MesheComp`) (`local.RowAndCol`) (`self.CheckID`)))
          (:`NewEnumerator1`
            (`self.CheckDef` (`local.MesheComp`) (`local.RowAndCol`) (`self.CheckID`) "OnWater"))))
      (:`then_1`
        ;[1 1 1] 返回检测结果，不等于-1则表示可以放置
        (bind _output_get (set `self.bPlay` (!= _playtargetline_row -1)))
        (set `self.bCardSelect` _output_get)))))

(fn `Check Hor`
  (params (MesheComp :type "MesheControllComponent Object Reference") (RowAndCol :type "Line Structure") (ID :type Integer) (CheckRow :type Integer) (CheckMesheType :type "ELineType Enum" :default "OnGround"))
  (bind (_rowandcol_row _rowandcol_col) (break `Line` (`local.RowAndCol`)))
  (for _index (range _rowandcol_col)
    (bind _returnvalue (`MesheControllComponent.GetMapMesh` (`local.MesheComp`) (`local.CheckRow`) _index))
    (`/Engine/EditorBlueprintResources/StandardMacros.IsValid` (`MapMeshe.GetUIMapMeshe` _returnvalue)
      (:`Is Valid`
        (if (`|EnumEquality` "OnGround" (`local.CheckMesheType`))
          _))))
  (set `self.PlayTargetLine` (make `Line` -1 -1)))

(fn `Check Hor Meshe`
  (params (CheckRow :type Integer) (PlayType :type "ELineType Enum" :default "OnGround") (BeginIndex :type Integer) (EndIndex :type Integer :default 5))
  (locals (MesheComp :type "MesheControllComponent Object Reference") (RowAndCol :type "Line Structure"))
  (if (not (`self.bPlay`))
    (`self.Check Horizontal Range Group` (`|MakeArray` (make `/Game/Resource/BP/Data/CardData/DialogueChar/CheckHorizontal` (`local.CheckRow`) BeginIndex EndIndex)) PlayType)))

(fn `Check Horizontal Range Group`
  (params (Range :type "Array of /Game/Resource/BP/Data/CardData/DialogueChar/CheckHorizontal Structure") (CheckType :type "ELineType Enum" :default "OnGround"))
  (for _array_element Range
    (`self.Check Horizontal Range Meshe` _array_element CheckType)))

(fn `Check Horizontal Range Meshe`
  (params (CheckRange :type "/Game/Resource/BP/Data/CardData/DialogueChar/CheckHorizontal Structure") (CheckType :type "ELineType Enum" :default "OnGround"))
  (locals (LocalCol :type Integer))
  (bind (_checkrange_row _checkrange_begin _checkrange_end) (break `/Game/Resource/BP/Data/CardData/DialogueChar/CheckHorizontal` (`local.CheckRange`)))
  (bind _checkrange_row_2 (break `/Game/Resource/BP/Data/CardData/DialogueChar/CheckHorizontal` (`local.CheckRange`)))
  (if (not (`self.bPlay`))
    (for _index (range _checkrange_begin (+ _checkrange_end 1))
      (bind _output_get (set `local.LocalCol` _index))
      (bind _returnvalue (`MesheControllComponent.GetMapMesh` (`self.GetMesheComponent`) _checkrange_row_2 _output_get))
      (`/Engine/EditorBlueprintResources/StandardMacros.IsValid` (`MapMeshe.GetUIMapMeshe` _returnvalue)
        (:`Is Valid`
          (if (`|EnumEquality` "OnGround" (`local.CheckType`))
            _))))))

(fn `Check Vertical Range Group`
  (params (Range :type "Array of /Game/Resource/BP/Data/CardData/DialogueChar/CheckVertical Structure") (CheckType :type "ELineType Enum" :default "OnGround"))
  (for _array_element Range
    (`self.Check Vertical Range Meshe` _array_element CheckType)))

(fn `Check Vertical Range Meshe`
  (params (CheckRange :type "/Game/Resource/BP/Data/CardData/DialogueChar/CheckVertical Structure") (CheckType :type "ELineType Enum" :default "OnGround"))
  (locals (LocalRow :type Integer))
  (bind _checkrange_col (break `/Game/Resource/BP/Data/CardData/DialogueChar/CheckVertical` (`local.CheckRange`)))
  (bind (_checkrange_col_2 _checkrange_begin _checkrange_end) (break `/Game/Resource/BP/Data/CardData/DialogueChar/CheckVertical` (`local.CheckRange`)))
  (if (not (`self.bPlay`))
    (for _index (range _checkrange_begin (+ _checkrange_end 1))
      (bind _output_get (set `local.LocalRow` _index))
      (bind _returnvalue (`MesheControllComponent.GetMapMesh` (`self.GetMesheComponent`) _output_get _checkrange_col))
      (`/Engine/EditorBlueprintResources/StandardMacros.IsValid` (`MapMeshe.GetUIMapMeshe` _returnvalue)
        (:`Is Valid`
          (if (`|EnumEquality` "OnGround" (`local.CheckType`))
            _))))))

(fn `CheckDatasLen`
  (params (Datas :type "Map of String to /Game/Resource/BP/Data/CardData/DialogueChar/PlayCardStruct Structure (by ref)"))
  (returns (CheckResult :type Boolean))
  (return (> (`BlueprintMapLibrary.Map_Length` Datas) 0)))

(fn `CheckDef`
  (params (MesheComp :type "MesheControllComponent Object Reference") (RowAndCol :type "Line Structure") (ID :type Integer) (CheckMesheType :type "ELineType Enum" :default "OnGround"))
  (locals (TargetLine :type "Line Structure"))
  (bind (_rowandcol_row _rowandcol_col) (break `Line` (`local.RowAndCol`)))
  (for _index (range _rowandcol_col)
    (for _index_2 (range _rowandcol_row)
      ;[1 1 1] 顺序遍历 行列，查找空位
      (bind _returnvalue (`MesheControllComponent.GetMapMesh` (`local.MesheComp`) _index_2 _index))
      (bind _returnvalue_2 (`MapMeshe.GetUIMapMeshe` _returnvalue))
      (`/Engine/EditorBlueprintResources/StandardMacros.IsValid` _returnvalue_2
        (:`Is Valid`
          (if (`|EnumEquality` (`UI_MapMeshe.GetLineType` _returnvalue_2) (`local.CheckMesheType`))
            ;;[1 0 0] 如果存在角色，并且和角色ID重叠，则无法放置
            (if (`UI_MapMeshe.GetbHasPlayer` _returnvalue_2)
              (if (not (== (`local.ID`) 0))
                (`/Engine/EditorBlueprintResources/StandardMacros.IsValid` null :!label _label
                  (:`Is Not Valid`
                    (set `self.PlayTargetLine` (make `Line` _index_2 _index))
                    (return))))
              (else
                (goto _label))))))))
  (set `self.PlayTargetLine` (make `Line` -1 -1)))

(fn `CheckDoubleCondition`
  (params (B1 :type "Boolean (by ref)") (B2 :type "Boolean (by ref)") (CheckAndCondition :type Boolean))
  (returns (ReturnValue :type Boolean))
  (bind _returnvalue (== B1 B2))
  (if _returnvalue
    (if (== _returnvalue CheckAndCondition)
      (return true)
      (else
        (return false)))
    (else
      (return false))))

(fn `CheckIndexIsValid`
  (params (CheckIndex :type Integer) (CheckEnd :type Integer))
  (returns (ValidIndex :type Integer))
  (if (< CheckIndex 0)
    (return 0)
    (elif (>= CheckIndex CheckEnd)
      (return (- (`local.CheckEnd`) 1))
      (else
        (return (`local.CheckIndex`))))))

(fn `CheckMouse`
  (returns (ValidMouse :type Boolean))
  (`GameMapInstance.GetGameMapInstance`)
  (bind _returnvalue (`MouseManagerComponent.IsMouseExist` (`GameMapInstance.GetGameMapMouseManagerStatic`)))
  (return _returnvalue))

(fn `CheckMouseCount`
  (params (CheckCount :type Integer) (LessThan :type Boolean :default true))
  (returns (Result :type Boolean))
  (bind _outallmouse (`MouseManagerComponent.GetAllMouse` (`GameMapInstance.GetGameMapMouseManagerStatic`)))
  (if (`local.LessThan`)
    (bind _returnvalue (`KismetArrayLibrary.Array_Length` _outallmouse))
    (return (<= _returnvalue (`local.CheckCount`)))
    (else
      (return (>= (`local.CheckCount`) _returnvalue)))))

(fn `CheckMouseTopLocation`
  (params (LineType :type "ELineType Enum (by ref)"))
  (returns (MouseActor :type "MouseActor Object Reference") (Location :type "Vector Structure"))
  (bind _returnvalue (`MouseManagerComponent.GetTopMouseByType` (`GameMapInstance.GetGameMapMouseManagerStatic`) LineType))
  (return _returnvalue (`self.K2_GetActorLocation` _returnvalue)))

(fn `Get Horizontal Range`
  (params (Row :type Integer) (BeginIndex :type Integer) (EndIndex :type Integer))
  (returns (Range :type "/Game/Resource/BP/Data/CardData/DialogueChar/CheckHorizontal Structure"))
  (bind _returnvalue (`MesheControllComponent.GetMapMeshRowAndCol` (`self.GetMesheComponent`)))
  (return (make `/Game/Resource/BP/Data/CardData/DialogueChar/CheckHorizontal` (`self.CheckIndexIsValid` Row (break `Line` _returnvalue)) (`self.CheckIndexIsValid` BeginIndex (`.Col` (break `Line` _returnvalue))) (`self.CheckIndexIsValid` EndIndex (`.Col` (break `Line` _returnvalue))))))

(fn `Get Random Play Result`
  (params (Datas :type "Map of String to /Game/Resource/BP/Data/CardData/DialogueChar/PlayCardStruct Structure (by ref)"))
  (if (not (`self.bCardSelect`))
    (bind _keys (`BlueprintMapLibrary.Map_Keys` Datas))
    (bind _output_get (set `self.TargetPlayCardName` (`KismetArrayLibrary.Array_Random` _keys)))
    (bind _value (`BlueprintMapLibrary.Map_Find` (`local.Datas`) _output_get))
    (set `self.TargetPlayCardGrade` (break `/Game/Resource/BP/Data/CardData/DialogueChar/PlayCardStruct` _value))
    (set `self.CheckID` (`.ID_7_33C4901544F54C564BA731A4C0C85FE8` (break `/Game/Resource/BP/Data/CardData/DialogueChar/PlayCardStruct` _value)))
    (set `self.bCardSelect` true)))

(fn `Get Vertical Range`
  (params (Col :type Integer) (Begin :type Integer) (End :type Integer))
  (returns (Range :type "/Game/Resource/BP/Data/CardData/DialogueChar/CheckVertical Structure"))
  (bind _returnvalue (`MesheControllComponent.GetMapMeshRowAndCol` (`self.GetMesheComponent`)))
  (return (make `/Game/Resource/BP/Data/CardData/DialogueChar/CheckVertical` (`self.CheckIndexIsValid` Col (`.Col` (break `Line` _returnvalue))) (`self.CheckIndexIsValid` Begin (break `Line` _returnvalue)) (`self.CheckIndexIsValid` End (break `Line` _returnvalue)))))

(fn `GetCurrentSpawnMouseRow`
  (returns (Row :type Integer))
  (bind _returnvalue (`MouseManagerComponent.GetCurrentSpawnMouseRow` (`GameMapInstance.GetGameMapMouseManagerStatic`)))
  (return _returnvalue))

(fn `GetCurrentTopMouse`
  (params (LineType :type "ELineType Enum" :default "OnGround"))
  (returns (TopMouse :type "MouseActor Object Reference"))
  (bind _returnvalue (`MouseManagerComponent.GetTopMouseByType` (`GameMapInstance.GetGameMapMouseManagerStatic`) LineType))
  (return _returnvalue))

(fn `GetMesheComponent`
  (returns (Comp :type "MesheControllComponent Object Reference"))
  (return (`GameMapInstance.GetGameMapMesheControllManagerStatic`)))

(fn `InitPlayCardState`
  (set `self.bCardSelect` false)
  (set `self.PlayTargetLine` (make `Line` -1 -1))
  (set `self.TargetPlayCardGrade` 0)
  (set `self.TargetPlayCardName` "")
  (set `self.bPlay` false))

(fn `Play Card to Ground`
  (params (Datas :type "Map of String to /Game/Resource/BP/Data/CardData/DialogueChar/PlayCardStruct Structure"))
  (bind _validmouse (`self.CheckMouse`))
  (if _validmouse
    (bind (_spawn1 _atk_line1 _atk_proj1 _func_bomb1 _func_playbomb1 _defence_def1 _defence_safe1) (`self.CategroyCardsByGround` (`local.Datas`)))
    (`|ExecutionSequence`
      (:`then_0`
        (`self.Player Card To Any Spawn` _spawn1))
      (:`then_1`
        (`self.Player Card To Any Defence` _defence_def1))
      (:`then_2`
        (`self.Player Card To Any ATK` _atk_line1 _atk_proj1)
        (`self.Player Card To Any Safe` _defence_safe1)))
    (else
      ;[1 1 1] 如果场上没有任何老鼠(只会放置生产和防御卡)
      (bind (_spawn1_2 _atk_line1_2 _atk_proj1_2 _func_bomb1_2 _func_playbomb1_2 _defence_def1_2) (`self.CategroyCardsByGround` (`local.Datas`)))
      (if (`self.CheckDoubleCondition` (`self.CheckDatasLen` _spawn1_2) (`self.CheckDatasLen` _defence_def1_2) true)
        (if (`KismetMathLibrary.RandomBool`)
          (`self.Player Card To Any Spawn` _spawn1_2 :!label _label)
          (else
            (`self.Player Card To Any Defence` _defence_def1_2 :!label _label_2)))
        (elif (`self.CheckDatasLen` _spawn1_2)
          (goto _label)
          (else
            (goto _label_2)))))))

(fn `PlayCard`
  (bind (_playtargetline_row _playtargetline_col) (break `Line` (`self.PlayTargetLine`)))
  (bind _targetplaycardname (`self.TargetPlayCardName`))
  (bind _returnvalue (`KismetStringLibrary.Conv_IntToString` (`self.TargetPlayCardGrade`)))
  (if (`self.bCardSelect`)
    ;[1 1 1] 最终通过指令放置，目标防御卡
    (if (`self.bPlay`)
      (`GameSystemFunction.AddGameinstructions` self (`KismetStringLibrary.Concat_StrStr` "/game play " _targetplaycardname "," _returnvalue " " (`KismetStringLibrary.Conv_IntToString` _playtargetline_row) "," (`KismetStringLibrary.Conv_IntToString` _playtargetline_col)) false)
      (`KismetSystemLibrary.PrintString` (`KismetStringLibrary.Concat_StrStr` _returnvalue "：" _targetplaycardname))
      (else
        ;;[1 1 1] 不满足放置条件，重置卡片选择
        (set `self.bCardSelect` false)))))

(fn `Player Card To Any ATK`
  (params (DatasShootLine :type "Map of String to /Game/Resource/BP/Data/CardData/DialogueChar/PlayCardStruct Structure (by ref)") (DatasProj :type "Map of String to /Game/Resource/BP/Data/CardData/DialogueChar/PlayCardStruct Structure (by ref)") (CheckType :type "ELineType Enum" :default "OnGround"))
  (if (`self.bCardSelect`)
    _
    (elif (`self.CheckMouseCount` 10)
      (if (== (== (> (`BlueprintMapLibrary.Map_Length` (`local.DatasProj`)) 0) (> (`BlueprintMapLibrary.Map_Length` (`local.DatasShootLine`)) 0)) true)
        (if (`KismetMathLibrary.RandomBool`)
          (`self.Get Random Play Result` (`local.DatasProj`) :!label _label)
          (else
            (`self.Get Random Play Result` (`local.DatasShootLine`) :!label _label_2)))
        (bind _row (`self.GetCurrentSpawnMouseRow`))
        (`|ExecutionSequence`
          (:`then_0`
            (`self.Check Vertical Range Group` (`|MakeArray` (`self.Get Vertical Range` 1 _row _row) (`self.Get Vertical Range` 2 _row _row) (`self.Get Vertical Range` 3 _row _row) (`self.Get Vertical Range` 4 _row _row)) (`local.CheckType`)))
          (:`then_1`
            (bind _topmouse (`self.GetCurrentTopMouse` (`local.CheckType`)))
            (`/Engine/EditorBlueprintResources/StandardMacros.IsValid` _topmouse
              (:`Is Valid`
                (bind _returnvalue (`MouseActor.GetMouseLine` _topmouse))
                (`self.Check Hor Meshe` (break `Line` _returnvalue) (`local.CheckType`)))))
          (:`then_2`
            (`self.PlayCard`)))
        (elif (> (`BlueprintMapLibrary.Map_Length` (`local.DatasProj`)) 0)
          (goto _label)
          (elif (> (`BlueprintMapLibrary.Map_Length` (`local.DatasShootLine`)) 0)
            (goto _label_2)))))))

(fn `Player Card To Any Defence`
  (params (Datas :type "Map of String to /Game/Resource/BP/Data/CardData/DialogueChar/PlayCardStruct Structure (by ref)") (CheckType :type "ELineType Enum" :default "OnGround"))
  (if (`self.bCardSelect`)
    _
    (elif (> (`BlueprintMapLibrary.Map_Length` (`local.Datas`)) 0)
      (`self.Get Random Play Result` (`local.Datas`))
      (bind _validmouse (`self.CheckMouse`))
      (if _validmouse
        (bind _row (`self.GetCurrentSpawnMouseRow`))
        (`|ExecutionSequence`
          (:`then_0`
            (`self.Check Vertical Range Group` (`|MakeArray` (`self.Get Vertical Range` 8 _row _row)) (`local.CheckType`)))
          (:`then_2`
            (`self.PlayCard`)))
        (else
          (`self.Check Vertical Range Group` (`|MakeArray` (`self.Get Vertical Range` 8 0 20)) (`local.CheckType`))
          (`self.PlayCard`))))))

(fn `Player Card To Any Safe`
  (params (Datas :type "Map of String to /Game/Resource/BP/Data/CardData/DialogueChar/PlayCardStruct Structure (by ref)") (CheckType :type "ELineType Enum" :default "OnGround"))
  (if (`self.bCardSelect`)
    _
    (elif (> (`BlueprintMapLibrary.Map_Length` (`local.Datas`)) 0)
      (if (`self.CheckMouseCount` 15 false)
        (`self.Get Random Play Result` (`local.Datas`))
        (`|ExecutionSequence`
          (:`then_0`
            (bind _topmouse (`self.GetCurrentTopMouse` "Sky"))
            (`/Engine/EditorBlueprintResources/StandardMacros.IsValid` _topmouse
              (:`Is Valid`
                (bind _returnvalue (`MouseActor.GetMouseLine` _topmouse))
                (`self.Check Vertical Range Group` (`|MakeArray` (`self.Get Vertical Range` 0 (break `Line` _returnvalue) (break `Line` _returnvalue))) (`local.CheckType`)))))
          (:`then_1`
            (bind _topmouse_2 (`self.GetCurrentTopMouse` "Underwater"))
            (`/Engine/EditorBlueprintResources/StandardMacros.IsValid` _topmouse_2
              (:`Is Valid`
                (bind _returnvalue_2 (`MouseActor.GetMouseLine` _topmouse_2))
                (`self.Check Vertical Range Group` (`|MakeArray` (`self.Get Vertical Range` 0 (break `Line` _returnvalue_2) (break `Line` _returnvalue_2))) (`local.CheckType`)))))
          (:`then_2`
            (bind _row (`self.GetCurrentSpawnMouseRow`))
            (`self.Check Horizontal Range Group` (`|MakeArray` (`self.Get Horizontal Range` _row 5 7)) (`local.CheckType`))))))))

(fn `Player Card To Any Spawn`
  (params (Cards :type "Map of String to /Game/Resource/BP/Data/CardData/DialogueChar/PlayCardStruct Structure") (CheckType :type "ELineType Enum" :default "OnGround"))
  (if (not (`self.bCardSelect`))
    ;[1 1 1] 当老鼠小于0
    (if (`self.CheckMouseCount` 0)
      (if (> (`BlueprintMapLibrary.Map_Length` (`local.Cards`)) 0)
        (`self.Get Random Play Result` (`local.Cards`))
        (`|ExecutionSequence`
          (:`then_0`
            (`self.Check Vertical Range Group` (`|MakeArray` (`self.Get Vertical Range` 4 0 20) (`self.Get Vertical Range` 5 0 20) (`self.Get Vertical Range` 6 0 20)) (`local.CheckType`)))
          (:`then_2`
            (`self.PlayCard`)))))))

(fn `UserConstructionScript`
  (`parent.UserConstructionScript`))