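; Line-trace sensor actor for VS mode that detects mice or flying items crossing its line.
; Each tick it traces from its location to MDirection on a custom channel, with one-frame debug drawing.
; With ClearMouse set, a MouseActor hit calls GameFailed on the VS map manager unless the game is over.
; Otherwise, with ClearItem set, a FlyItemActor hit is returned to its pool.
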(event `self.BlueprintTick`
  (params (DeltaSeconds :type "Float (single-precision)"))
  (bind _outhit (`KismetSystemLibrary.LineTraceSingle` :`Start` (`self.K2_GetActorLocation`) :`End` (`self._M_Direction`) :`TraceChannel` "TraceTypeQuery11" :`DrawDebugType` "ForOneFrame"))
  (if (`self.ClearMouse`)
    (bind (_bblockinghit _binitialoverlap _time _distance _location _impactpoint _normal _impactnormal _physmat _hitactor) (`GameplayStatics.BreakHitResult` _outhit))
    (cast `MouseActor` _hitactor)
    (if (not (`GameStartSubsystem.GetbGameOver`))
      (`GameMapInstance.GetGameMapInstance`)
      (`VSManagerComponent.GameFailed` (`GameMapInstance.GetGameMapVsManagerStatic`)))
    (elif (`self.ClearItem`)
      (bind _asfly_item_actor (cast `FlyItemActor` _hitactor))
      (`FlyItemActor.ReturnPool` _asfly_item_actor))))

(fn `UserConstructionScript`)