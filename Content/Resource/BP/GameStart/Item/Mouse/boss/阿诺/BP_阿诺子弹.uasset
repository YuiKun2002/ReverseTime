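; Projectile for the mouse boss 阿诺 (Anuo) that lobs toward a target location in an arc.
; InitTarget stores start and target points, and a timeline feeds two curves into an arc helper to move the actor.
; On landing, unless the game is over, it plays a bomb flipbook, self-destroys and sphere-traces for CardActors.
; The KillCard logic is disconnected, so hit cards are unaffected.
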(event `self.ReceiveBeginPlay`
  (`self.InitRotation`)
  (`self.SetFlipbookPitchRotation` 17.0)
  (add `self.Run` (delegate `CustomEvent_0`)))

(event `CustomEvent_0`
  (bind _returnvalue (`self.K2_GetActorLocation`))
  (bind (_direction _newtrack_0 _newtrack_1) (`Timeline|Timeline_0` :!via `PlayFromStart`)
    (:`Update`
      (bind _outlocation (`GameSystemFunction.GetCurveLineByTimeLineBlue` (`self.Cur Location`) (`self.Target Location`) 40.0 _newtrack_0 _newtrack_1))
      (`self.K2_SetActorLocation` _outlocation))
    (:`Finished`
      (if (not (`self.GetbGameOver`))
        (`self.SetFlipbookPitchRotation` 0.0)
        (`self.SetPlayAnimation` "/Game/Resource/Texture/Sprite/VS/Sprite/Mouse/Boss/阿诺/FB_Bomb.FB_Bomb")
        (`self.SetAnimationPlayEndDestroy`)
        (bind (_outhits _returnvalue_2) (`KismetSystemLibrary.SphereTraceMulti` :`Start` _returnvalue :`End` _returnvalue :`Radius` 15.0 :`TraceChannel` "TraceTypeQuery3" :`DrawDebugType` "ForDuration"))
        (if _returnvalue_2
          (for _array_element _outhits
            (bind _ascard_actor (cast `CardActor` (`.HitActor` (`GameplayStatics.BreakHitResult` _array_element))))))))))

(fn `InitTarget`
  (params (TargetLocation :type "Vector Structure") (CurLocation :type "Vector Structure"))
  (set `self.Target Location` TargetLocation)
  (set `self.Cur Location` CurLocation))

(fn `UserConstructionScript`)