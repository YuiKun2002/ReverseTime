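; Bandage Blueprint for the Pharaoh mouse boss, a short-lived mouse actor that expires on a timer.
; On BeginPlay it plays a default flipbook animation once, with a finish animation set to follow.
; Tick counts down Time, then flags the mouse dead a single time through SetMouseDeath.
; The OnDeathed event calls MouseKill and destroys the actor.
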(event `self.ReceiveBeginPlay`
  (`FlipbookBaseComponent.SetPlayAnimationOnce` (`self.M_Actor`) "/Game/Resource/Texture/Sprite/VS/Sprite/Mouse/Boss/法老/silkworm/FB_Def.FB_Def" "/Game/Resource/Texture/Sprite/VS/Sprite/Mouse/Boss/法老/silkworm/FB_Finish.FB_Finish"))

(event `self.BlueprintTick`
  (params (DeltaSeconds :type "Float (single-precision)"))
  (if (> (`self.time`) 0.0)
    (set `self.time` (- (`self.time`) DeltaSeconds))
    (elif (not (`self.bDeath`))
      (set `self.bDeath` true)
      (`self.SetMouseDeath` true))))

(event `self.OnDeathed`
  (`self.MouseKill`)
  (`self.K2_DestroyActor`))

(fn `UserConstructionScript`)