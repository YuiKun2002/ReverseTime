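; Pipe entrance (管道入口) actor for the 洞君 mouse boss, placed on a map grid cell.
; Init snaps it to the map mesh at its Line row and column; BeginPlay sets rotation and runs a timeline driving material parameter "A" from 0 to 1.
; The animation-end event reveals a sorted ground sprite when InWater is true.
; The branch choosing water or ground animations, setting InWater and offsetting position is disconnected and never runs.
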(event `self.OnAnimationPlayEndBlueprint`
  (if (`self.inWater`)
    (`SceneComponent.SetHiddenInGame` (`self.F_M_B_0_Ground_2`) false false)
    (`PrimitiveComponent.SetTranslucentSortPriority` (`self.F_M_B_0_Ground_2`) (+ (`self.Layer`) 1))))

(event `self.ReceiveBeginPlay`
  (`self.InitRotation`)
  (bind (_direction _newtrack_0) (`Timeline|Timeline_0` :!via `PlayFromStart`)
    (:`Update`
      (`MeshComponent.SetScalarParameterValueOnMaterials` (`self.M_Actor`) "A" (`KismetMathLibrary.Lerp` 0.0 1.0 _newtrack_0)))))

(fn `Init`
  (params (Line :type "Line Structure"))
  (locals (Ins :type "GameMapInstance Object Reference"))
  (bind (_line_row _line_col) (break `Line` (`local.Line`)))
  (bind _returnvalue (`GameMapInstance.GetGameMapInstance`))
  (`/Engine/EditorBlueprintResources/StandardMacros.IsValid` _returnvalue
    (:`Is Valid`
      (set `local.Ins` _returnvalue)
      (bind _returnvalue_2 (`MesheControllComponent.GetMapMesh` (`GameMapInstance.GetGameMapMesheControllManagerStatic`) _line_row _line_col))
      (`self.K2_SetActorLocation` (`self.K2_GetActorLocation` _returnvalue_2))
      (set `self.Location` (`self.K2_GetActorLocation`)))))

(fn `UserConstructionScript`)