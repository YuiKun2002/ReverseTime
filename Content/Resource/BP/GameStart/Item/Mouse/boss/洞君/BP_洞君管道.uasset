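; Pipe for the 洞君 mouse boss, pairing a spawned entrance actor with this actor's exit on the map grid.
; InitChannelin spawns and places the BP_管道入口 entrance; InitChannelOut plays the ground animation, passes on the cell's line type, then calls End when the animation finishes.
; Hits switch to a damaged animation at half HP, and Hidde fades and scales the mesh by timeline.
; Destruction also removes the entrance; the fade-in timeline is unwired.
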(event `self.InitChannelIn`
  (params (NewLine :type "Line Structure"))
  (`/Engine/EditorBlueprintResources/StandardMacros.IsValid` (`self.InChannelActor`)
    (:`Is Valid`
      (set `self.bEnd` false))
    (:`Is Not Valid`
      (bind _returnvalue (`|SpawnActorFromClass` "/Game/Resource/BP/GameStart/Item/Mouse/boss/洞君/BP_管道入口.BP_管道入口_C" (`KismetMathLibrary.MakeTransform` (0.0 0.0 0.0)) "Undefined" "OverrideRootScale" null null))
      (`/Game/Resource/BP/GameStart/Item/Mouse/boss/洞君/BP_管道入口.Init` _returnvalue (make `Line` NewLine_Row NewLine_Col))
      (set `self.InChannelActor` _returnvalue)
      (set `self.bEnd` false))))

(event `self.InitChannelOut`
  (params (NewLine :type "Line Structure"))
  (bind _returnvalue (`MesheControllComponent.GetMapMesh` (`GameMapInstance.GetGameMapMesheControllManagerStatic`) NewLine_Row NewLine_Col))
  (`FlipbookBaseComponent.SetPlayAnimationOnce` (`self.M_Actor`) "/Game/Resource/Texture/Sprite/VS/Sprite/Mouse/Boss/0/Anim/F_M_B_0_Ground.F_M_B_0_Ground" "/Game/Resource/Texture/Sprite/VS/Sprite/Mouse/Boss/0/Anim/F_M_B_0_Ground_Def.F_M_B_0_Ground_Def")
  (`self.BPInMapMeshe` (`MapMeshe.GetLineType` _returnvalue))
  (set `self.bEnd` true))

(event `self.OnAnimationPlayEndBlueprint`
  (if (`self.bEnd`)
    (set `self.bEnd` false)
    (`self.End`)))

(event `self.Hidde`
  (bind (_direction _newtrack_0 _newtrack_1) (`Timeline|Timeline_0` :!via `PlayFromStart`)
    (:`Update`
      (`MeshComponent.SetScalarParameterValueOnMaterials` (`self.M_Actor`) "A" (`KismetMathLibrary.Lerp` 1.0 0.0 _newtrack_0))
      (`SceneComponent.SetRelativeScale3D` (`self.M_Actor`) _newtrack_1))))

(event `self.BPBeHit`
  (params (CurHP :type "Float (single-precision)") (TotalHP :type "Float (single-precision)"))
  (if (> CurHP (* TotalHP 0.5))
    (`FlipbookBaseComponent.SetPlayAnimation` (`self.M_Actor`) "/Game/Resource/Texture/Sprite/VS/Sprite/Mouse/Boss/0/Anim/F_M_B_0_Ground_Def.F_M_B_0_Ground_Def" false)
    (else
      (`FlipbookBaseComponent.SetPlayAnimation` (`self.M_Actor`) "/Game/Resource/Texture/Sprite/VS/Sprite/Mouse/Boss/0/Anim/F_M_B_0_Ground_Low.F_M_B_0_Ground_Low" false))))

(event `self.ReceiveDestroyed`
  (`self.K2_DestroyActor` (`self.InChannelActor`)))

(fn `UserConstructionScript`)