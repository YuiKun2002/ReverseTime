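; Missile fired by the 轰隆隆 mouse boss that kills player cards where it lands.
; It climbs on Tick while GetResult is false; when a first timeline ends, InitLocation runs and a second timeline drives UpdatePosition.
; On arrival it switches to its end animation with destroy-on-finish and flips the flipbook pitch.
; A small sphere trace then calls KillCard and ResourceAddBadCard for each CardActor hit.
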(event `self.ReceiveBeginPlay`
  (bind _returnvalue (`self.K2_GetActorLocation`))
  (`Timeline|Timeline_0`
    (:`Finished`
      (`self.InitLocation`)
      (bind (_direction _newtrack_0) (`Timeline|Timeline_1`)
        (:`Update`
          (`self.UpdatePosition` _newtrack_0))
        (:`Finished`
          (`self.SetPlayAnimation` "/Game/Resource/Texture/Sprite/VS/Sprite/Mouse/Boss/1/Anim/Attack_1_state1_3.Attack_1_state1_3")
          (`self.SetAnimationPlayEndDestroy`)
          (`self.SetFlipbookPitchRotation` -180.0)
          (bind _outhits (`KismetSystemLibrary.SphereTraceMulti` :`Start` _returnvalue :`End` (+ _returnvalue (0.0 0.0 15.0)) :`Radius` 25.0 :`TraceChannel` "TraceTypeQuery3" :`DrawDebugType` "ForOneFrame"))
          (for _array_element _outhits
            (bind _ascard_actor (cast `CardActor` (`.HitActor` (`GameplayStatics.BreakHitResult` _array_element))))
            (`CardActor.KillCard` _ascard_actor)
            (`ResourceManagerComponent.ResourceAddBadCard`)))))))

(event `self.BlueprintTick`
  (params (DeltaSeconds :type "Float (single-precision)"))
  (bind _returnvalue (`self.GetResult`))
  (if (not _returnvalue)
    (`self.K2_AddActorLocalOffset` (`KismetMathLibrary.MakeVector` 0.0 0.0 (* DeltaSeconds 200.0)))))

(fn `UserConstructionScript`)