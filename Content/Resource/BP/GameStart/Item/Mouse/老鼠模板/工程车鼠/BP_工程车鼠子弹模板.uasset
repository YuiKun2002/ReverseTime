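; Projectile template for the engineer-vehicle mouse (工程车鼠), lobbed at a target location on the card grid.
; Init stores the target, then a FlyTarget timeline moves the actor along an arc built from time and height curves.
; On landing, unless the game is over, it checks for living cards, plays the split animation and self-destroys, sphere-tracing if none are found.
; The KillCard and bad-card recording nodes are disconnected, so impact damages nothing here.
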(event `self.Init`
  (params (TargetLocation :type "Vector Structure (by ref)") (TargetHitCard :type "Array of CardActor Object Reference (by ref)"))
  (bind _returnvalue (`self.K2_GetActorLocation`))
  ;[1 1 1] 初始化条件以及位置信息
  (set `self.Target Location` TargetLocation)
  (set `self.Target Hit Card` TargetHitCard)
  (set `self.CurLocation` (`self.K2_GetActorLocation`))
  (set `self.bHit` false)
  ;[1 1 1] 从起始点飞向目标点的抛物线
  (bind (_direction _locationtime _highttime) (`Timeline|FlyTarget` :!via `PlayFromStart`)
    (:`Update`
      (bind _outlocation (`GameSystemFunction.GetCurveLineByTimeLineBlue` (`self.CurLocation`) (`self.Target Location`) 120.0 _locationtime _highttime))
      (`self.K2_SetActorLocation` _outlocation))
    (:`Finished`
      ;[1 1 1] 如果当前网格存在的卡片有效，则直接消耗血量，死亡则记录卡片损坏
      (if (not (`self.GetbGameOver`))
        (for _array_element _
          (`/Engine/EditorBlueprintResources/StandardMacros.IsValid` _array_element
            (:`Is Valid`
              (if (> (`CardActor.GetCurrentHP` _array_element) 0.0)
                (set `self.bHit` true)))))
        (if (`self.bHit`)
          (`self.SetPlayAnimation` (`self.SplitAnim`))
          (`self.SetAnimationPlayEndDestroy`)
          (else
            ;[1 1 1] 之前的卡片全部都失效了，则临时创建球体范围检测，检测当前网格存在的卡片，并且消耗当前卡片的血量
            (`self.SetPlayAnimation` (`self.SplitAnim`))
            (`self.SetAnimationPlayEndDestroy`)
            (bind _outhit (`KismetSystemLibrary.SphereTraceSingle` :`Start` _returnvalue :`End` _returnvalue :`Radius` 20.0 :`TraceChannel` "TraceTypeQuery3" :`DrawDebugType` "ForDuration"))
            (bind _ascard_actor (cast `CardActor` (`.HitActor` (`GameplayStatics.BreakHitResult` _outhit))))
            (if (> (`CardActor.GetCurrentHP` _ascard_actor) 0.0)
              _)))))))

(event `self.ReceiveBeginPlay`
  (`self.InitRotation`))

(fn `UserConstructionScript`)