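; Blueprint for the 轰隆隆 mouse boss, providing its missile, laser and area attacks.
; Tick mirrors the water animation's visibility onto the base flipbook.
; A looping timer spawns three offset missiles; the laser spawns an actor and scans its grid row plus the preceding one.
; Sphere traces find nearby cards, but card removal, bad-card penalties and missile targeting are unwired, so scans have no effect.
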(event `self.BlueprintTick`
  (params (DeltaSeconds :type "Float (single-precision)"))
  ;[1 1 1] 水中动画
  (if (`SceneComponent.bHiddenInGame` (`self.InWaterAnim`))
    (if (not (`SceneComponent.bHiddenInGame` (`self.FlipbookBase`)))
      (`SceneComponent.SetHiddenInGame` (`self.FlipbookBase`) true false))
    (elif (`SceneComponent.bHiddenInGame` (`self.FlipbookBase`))
      (`SceneComponent.SetHiddenInGame` (`self.FlipbookBase`) false false))))

(event `self.OnSpawnMissile`
  (params (Location :type "Vector Structure"))
  (set `self.Location` Location)
  (set `self.SpawnCount` 3)
  (bind _returnvalue (`KismetSystemLibrary.K2_SetTimerDelegate` (delegate `Spawn`) 0.2 true))
  (set `self.Timer` _returnvalue))

(event `Spawn`
  (bind _returnvalue (+ (`self.Location`) (`|GetArrayItem` (`self.LocationOffset`) (`self.SpawnCount`))))
  (bind _output_get (set `self.SpawnCount` (- (`self.SpawnCount`) 1)))
  (if (<= _output_get 0)
    (`self.SpawnMissileLocation` _returnvalue)
    (`KismetSystemLibrary.K2_ClearAndInvalidateTimerHandle` (`self.Timer`))
    (else
      (`self.SpawnMissileLocation` _returnvalue))))

(event `self.OnSpawnLaser`
  (params (Location :type "Vector Structure"))
  (bind _returnvalue (`|SpawnActorFromClass` "/Game/Resource/BP/GameStart/Item/Mouse/boss/轰隆隆/BP_轰隆隆激光.BP_轰隆隆激光_C" (`KismetMathLibrary.MakeTransform` (0.0 0.0 0.0)) "DontSpawnIfColliding" "OverrideRootScale" null null))
  (`self.K2_SetActorLocation` _returnvalue (+ Location (0.0 -88.0 29.0)) false false)
  (bind _returnvalue_2 (`self.GetMouseLine`))
  (`self.SpawnLine` (break `Line` _returnvalue_2))
  (if (not (== (break `Line` _returnvalue_2) 0))
    (`self.SpawnLine` (- (break `Line` _returnvalue_2) 1))))

(event `self.SpawnRange`
  (`self.SpawnBox` (0.0 23.0 25.0))
  (`self.SpawnBox` (0.0 -23.0 25.0))
  (`self.SpawnBox` (0.0 23.0 25.0))
  (`self.SpawnBox` (0.0 -23.0 25.0))
  (`self.SpawnBox` (0.0 23.0 25.0))
  (`self.SpawnBox` (0.0 -23.0 25.0)))

(fn `SpawnBox`
  (params (Offset :type "Vector Structure"))
  (locals (NewLocalVar_2 :type "Float (single-precision)" :default 0.0))
  (bind _returnvalue (+ (`self.K2_GetActorLocation`) Offset))
  (bind (_outhits _returnvalue_2) (`KismetSystemLibrary.SphereTraceMulti` :`Start` _returnvalue :`End` _returnvalue :`Radius` 45.0 :`TraceChannel` "TraceTypeQuery3" :`DrawDebugType` "ForDuration"))
  (if _returnvalue_2
    (for _array_element _outhits
      (bind _ascard_actor (cast `CardActor` (`.HitActor` (`GameplayStatics.BreakHitResult` _array_element))))
      (`/Engine/EditorBlueprintResources/StandardMacros.IsValid` _ascard_actor))))

(fn `SpawnLine`
  (params (Row :type Integer))
  (locals (NewLocalVar_0 :type Integer :default 0) (NewLocalVar_1 :type "Float (single-precision)" :default 0.0) (NewLocalVar_3 :type "Array of EObjectTypeQuery Enum"))
  (bind _returnvalue (`GameMapInstance.GetGameMapMesheControllManagerStatic`))
  (bind _returnvalue_2 (`MesheControllComponent.GetMapMeshRowAndCol` _returnvalue))
  (for _index (range (`local.NewLocalVar_0`) (`.Col` (break `Line` _returnvalue_2)))
    (bind _returnvalue_3 (`MesheControllComponent.GetMapMesh` _returnvalue Row _index))
    (`/Engine/EditorBlueprintResources/StandardMacros.IsValid` (`MapMeshe.GetUIMapMeshe` _returnvalue_3))))

(fn `SpawnMissileLocation`
  (params (NewLocation :type "Vector Structure"))
  (bind _returnvalue (`|SpawnActorFromClass` "/Game/Resource/BP/GameStart/Item/Mouse/boss/轰隆隆/BP_轰隆隆导弹.BP_轰隆隆导弹_C" (`KismetMathLibrary.MakeTransform` (0.0 0.0 0.0)) "DontSpawnIfColliding" "OverrideRootScale" null null))
  (`self.InitRotation` _returnvalue)
  (`self.K2_SetActorLocation` _returnvalue NewLocation false false))

(fn `UserConstructionScript`)