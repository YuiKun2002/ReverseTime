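; Catfish mouse bomb projectile that lobs itself at a card tile in its row, falling back to the row's current left tile.
; A timeline drives the CruveMove arc, then plays the bomb animation.
; Animation-end callbacks offset and rescale it, then run a sphere trace and destroy it.
; Trace hits are cast to CardActor, but the KillCard and ResourceAddBadCard logic is disconnected, so nothing is killed.
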(event `self.ReceiveBeginPlay`
  (`self.InitRotation`))

(event `self.OnInit`
  (bind _targetlocation (`self.GenTargetLocation`))
  (`CruveMoveComponent.Cruve_Init` (`self.CruveMove`) (`self.K2_GetActorLocation`) _targetlocation 90.0)
  (bind (_direction _move _hight) (`Timeline|Timeline_0` :!via `PlayFromStart`)
    (:`Update`
      (`CruveMoveComponent.Curve_UpdateLocation` (`self.CruveMove`) self _move _hight))
    (:`Finished`
      (`FlipbookBaseComponent.SetPlayAnimationOnce` (`self.M_Actor`) "/Game/Resource/Texture/Sprite/VS/Sprite/Mouse/Mouse_1/普通/海底/鲶鱼老鼠/FB_鲶鱼老鼠炸弹.FB_鲶鱼老鼠炸弹" "/Game/Resource/Texture/Sprite/VS/Sprite/Items/20/Fly_Bomb.Fly_Bomb")
      (set `self.Start` true))))

(event `self.OnAnimationPlayEndBlueprint`
  (bind _returnvalue (`self.K2_GetActorLocation`))
  (if (`self.Start`)
    (`SceneComponent.K2_AddLocalOffset` (`self.M_Actor`) (-70.0 0.0 -37.0) false false)
    (if (`self.bPlay`)
      (bind _outhits (`KismetSystemLibrary.SphereTraceMulti` :`Start` _returnvalue :`End` _returnvalue :`Radius` 10.0 :`TraceChannel` "TraceTypeQuery3" :`DrawDebugType` "ForOneFrame"))
      (for _array_element _outhits
        (bind _ascard_actor (cast `CardActor` (`.HitActor` (`GameplayStatics.BreakHitResult` _array_element)))))
      (`self.K2_DestroyActor`)
      (else
        (set `self.bPlay` true)
        (`self.SetActorScale3D` (0.6 0.6 0.6))))))

(fn `GenTargetLocation`
  (returns (TargetLocation :type "Vector Structure"))
  (bind _returnvalue (`GameMapInstance.GetGameMapMesheControllManagerStatic`))
  (bind _returnvalue_2 (`self.GetLine`))
  (bind _returnvalue_3 (`MesheControllComponent.GetHasCardMeshe` _returnvalue (break `Line` _returnvalue_2)))
  (`/Engine/EditorBlueprintResources/StandardMacros.IsValid` _returnvalue_3
    (:`Is Valid`
      (return (`self.K2_GetActorLocation` _returnvalue_3)))
    (:`Is Not Valid`
      (bind _returnvalue_4 (`MesheControllComponent.GetMapMeshCurrentLeft` _returnvalue (break `Line` _returnvalue_2)))
      (`/Engine/EditorBlueprintResources/StandardMacros.IsValid` _returnvalue_4
        (:`Is Valid`
          (return (`self.K2_GetActorLocation` _returnvalue_4)))
        (:`Is Not Valid`
          (return (0.0 0.0 0.0)))))))

(fn `UserConstructionScript`)