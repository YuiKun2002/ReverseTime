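; Template Blueprint for a mouse hole (老鼠洞), a mouse-side item that spawns a companion grid actor.
; BeginPlay plays the generation animation; when it first ends, it calls OnInit and spawns BP老鼠洞网格 at its location, passing its line and a self-reference.
; While alive and initialized, it forwards Tick through CallTick, or marks itself dead if the grid actor becomes invalid.
; Destroying the hole also destroys the grid actor.
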(event `self.ReceiveBeginPlay`
  ;[1 1 1] 播放老鼠洞动画
  (`self.SetPlayAnimationOnce` "/Game/Resource/Texture/Sprite/VS/Sprite/Mouse/Boss/法老/老鼠洞/t/FB_Gen.FB_Gen" "/Game/Resource/Texture/Sprite/VS/Sprite/Mouse/Boss/法老/老鼠洞/t/FB_Finish.FB_Finish")
  (set `self.bInit` false)
  (set `self.bTickInit` false))

(event `self.OnAnimationPlayEndBlueprint`
  ;[1 1 1] 当老鼠洞动画播放完毕后，进行初始化生成
  (if (not (`self.bInit`))
    (set `self.bInit` true)
    (set `self.bTickInit` true)
    (`self.OnInit`)
    (bind _returnvalue (`|SpawnActorFromClass` "/Game/Resource/BP/GameStart/VS/CustomMeshe/custom/BP老鼠洞网格.BP老鼠洞网格_C" (`KismetMathLibrary.MakeTransform` (`self.K2_GetActorLocation`)) "Undefined" "OverrideRootScale" null null))
    (bind _output_get (set `self.MouseBlockActor` _returnvalue))
    (bind _returnvalue_2 (`self.GetMouseLine`))
    (`CustomMapMeshe.SetLine` _output_get _returnvalue_2)
    (set `/Game/Resource/BP/GameStart/VS/CustomMeshe/custom/BP老鼠洞网格.老鼠洞模板` self _returnvalue)))

(event `self.ReceiveDestroyed`
  (bind _mouseblockactor (`self.MouseBlockActor`))
  ;[1 1 1] 当前对象被销毁时，一并销毁老鼠洞对象
  (if (`KismetSystemLibrary.IsValid` _mouseblockactor)
    (`self.K2_DestroyActor` _mouseblockactor)))

(event `self.BlueprintTick`
  (params (DeltaSeconds :type "Float (single-precision)"))
  ;[1 1 1] 老鼠洞本身有效才会更新，否则直接销毁
  (bind _returnvalue (`self.GetMouseIsDeath`))
  (if _returnvalue
    _
    (elif (`self.bInit`)
      (if (`KismetSystemLibrary.IsValid` (`self.MouseBlockActor`))
        (if (`self.bTickInit`)
          (`self.Tick` DeltaSeconds))
        (else
          (`self.SetMouseDeath` true))))))

(fn `UserConstructionScript`)