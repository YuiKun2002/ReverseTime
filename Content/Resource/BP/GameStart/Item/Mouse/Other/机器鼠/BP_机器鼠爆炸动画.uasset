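; Robot mouse (机器鼠) explosion animation actor that plays a bomb sound on init and destroys itself when its animation ends.
; On init it sets its rotation and runs a radius multi-sphere trace at its location, with debug drawing, casting each hit actor to CardActor.
; The kill-card and bad-card resource logic is disconnected, so the explosion currently has no effect on the cards it hits.
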(event `self.OnInit`
  (bind _returnvalue (`self.K2_GetActorLocation`))
  (`self.InitRotation`)
  (`FVMGameInstance.PlayBGM_S_Static` "Bomb" "ItemAudio")
  (bind (_outhits _returnvalue_2) (`KismetSystemLibrary.SphereTraceMulti` :`Start` _returnvalue :`End` _returnvalue :`Radius` 100.0 :`TraceChannel` "TraceTypeQuery3" :`DrawDebugType` "ForDuration"))
  (if _returnvalue_2
    (for _array_element _outhits
      (bind _ascard_actor (cast `CardActor` (`.HitActor` (`GameplayStatics.BreakHitResult` _array_element))))))
  (`self.SetAnimationPlayEndDestroy`))

(fn `UserConstructionScript`)