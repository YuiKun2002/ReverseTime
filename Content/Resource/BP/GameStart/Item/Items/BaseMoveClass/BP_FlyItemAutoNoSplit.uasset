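; BP_FlyItemAutoNoSplit is a pooled homing projectile that chases targets, with comments indicating mice, and returns to its pool on hit.
; Its AutoTrackShoot component resets location and starts on init, then stops on hit or return, with its tickable-when-paused flag toggled on init and return.
; Tick accumulates time while the component has no target and recycles the projectile after a brief timeout.
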(event `self.OnHit`
  (params (AttackType :type "EFlyItemAttackType Enum" :default "Def"))
  ;[1 1 1] 当击中老鼠时，返回对象池
  (`AutoTrackShootComponent.Stop` (`self.AutoTrackShoot`))
  (`self.ReturnPool`)
  (set `self.Delta Seconds` 0.0))

(event `self.OnInit`
  (bind _autotrackshoot (`self.AutoTrackShoot`))
  ;[1 1 1] 从对象池取出，初始化时
  (`ActorComponent.SetTickableWhenPaused` _autotrackshoot false)
  (`AutoTrackShootComponent.InitLocation` _autotrackshoot)
  (`AutoTrackShootComponent.Start` _autotrackshoot)
  (set `self.Delta Seconds` 0.0))

(event `self.OnReturn`
  (bind _autotrackshoot (`self.AutoTrackShoot`))
  ;[1 1 1] 当需要返回对象池时
  (`ActorComponent.SetTickableWhenPaused` _autotrackshoot true)
  (`AutoTrackShootComponent.Stop` _autotrackshoot))

(event `self.BlueprintTick`
  (params (DeltaSeconds :type "Float (single-precision)"))
  ;[1 1 1] 飞行物没有追击目标时
  (bind _returnvalue (`AutoTrackShootComponent.GetTarget` (`self.AutoTrackShoot`)))
  (if _returnvalue
    (set `self.Delta Seconds` 0.0)
    (else
      (bind _output_get (set `self.Delta Seconds` (+ (`self.Delta Seconds`) DeltaSeconds)))
      (if (>= _output_get 0.2)
        (`self.ReturnPool`)))))

(fn `UserConstructionScript`)