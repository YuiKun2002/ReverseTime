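; Detail object for editing a defence card item in the item ID manager, holding one item's data for property editing.
; On init it casts the UI row and owning defence editor, then looks up the item's data by ID in the editor's Items map.
; When a property changes, SaveDetail pushes the data back to the linked UI item and tells it to save.
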(event `/Game/Resource/BP/Data/ItemIdManager/Property/0Base/BP_ItemID_Edit_PropertyInterface.InitDetailClass`
  (params (Owner :type "Object Object Reference") (UI :type "EditorUtilityWidget Object Reference") (Id :type Integer))
  ;[1 1 1] 初始化关联UI项，和初始化物品数据
  (bind _asbp_0_ui_item_id_edit_defence (cast `/Game/Resource/BP/Data/ItemIdManager/Property/Card/防御卡片/BP_0_UI_ItemID_Edit_Defence` UI))
  (set `self.As BP 0 UI Item ID Edit Defence` _asbp_0_ui_item_id_edit_defence)
  (bind _asbp_0_edit_item_id_defence (cast `/Game/Resource/BP/Data/ItemIdManager/Property/Card/防御卡片/BP_0_Edit_ItemID_Defence` Owner))
  (set `self.Data` (`BlueprintMapLibrary.Map_Find` (`/Game/Resource/BP/Data/ItemIdManager/Property/Card/防御卡片/BP_0_Edit_ItemID_Defence.Items` _asbp_0_edit_item_id_defence) Id)))

(event `/Game/Resource/BP/Data/ItemIdManager/Property/0Base/BP_ItemID_Edit_PropertyInterface.SaveDetail`
  (bind _as_bp_0_ui_item_id_edit_defence (`self.As BP 0 UI Item ID Edit Defence`))
  ;[1 1 1] 当属性发生变化时，自动触发，设置UI项中Data数据，随后让UI进行保存操作
  (set `/Game/Resource/BP/Data/ItemIdManager/Property/Card/防御卡片/BP_0_UI_ItemID_Edit_Defence.Data` (`self.Data`) _as_bp_0_ui_item_id_edit_defence)
  (`/Game/Resource/BP/Data/ItemIdManager/Property/0Base/BP_ItemID_Edit_PropertyInterface.SaveProperty` _as_bp_0_ui_item_id_edit_defence))