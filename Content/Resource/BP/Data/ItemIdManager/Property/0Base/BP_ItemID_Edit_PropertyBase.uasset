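; Base class for an item ID editor's data-table properties, caching row names, IDs and display names for listing, search and lookup.
; Events push the full cache or a row-name substring match to the Editor's UI, request new row widgets, and resolve an ID to its row name.
; The three collections are matched by index after ToArray.
; DataTableRowFind and GetDataRowName are placeholder stubs.
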(event `/Game/Resource/BP/Data/ItemIdManager/Property/0Base/BP_ItemID_Edit_PropertyInterface.ClassInit`
  ;[1 1 1] 初始化
  (`BlueprintSetLibrary.Set_Clear` (`self.Names`))
  (`BlueprintSetLibrary.Set_Clear` (`self.IDs`))
  (`BlueprintSetLibrary.Set_Clear` (`self.RowNames`)))

(event `/Game/Resource/BP/Data/ItemIdManager/Property/0Base/BP_ItemID_Edit_PropertyInterface.DataTableQuery`
  (params (KeyWords :type Text) (Editor :type "/Game/Resource/BP/Data/ItemIdManager/Editor/BP_核心数据表修改器 Object Reference") (SoftClassPath :type "SoftClassPath Structure"))
  ;[1 1 1] 查询
  ;;[1 1 1] 清理缓存
  (`BlueprintSetLibrary.Set_Clear` (`self.Query_RowNames`))
  (`BlueprintSetLibrary.Set_Clear` (`self.Query_IDs`))
  (`BlueprintSetLibrary.Set_Clear` (`self.QueryNames`))
  ;;[1 1 1] 查询关键词
  (bind _result (`BlueprintSetLibrary.Set_ToArray` (`self.Names`)))
  (bind _result_2 (`BlueprintSetLibrary.Set_ToArray` (`self.IDs`)))
  (bind _result_3 (`BlueprintSetLibrary.Set_ToArray` (`self.RowNames`)))
  (for (_array_element _array_index) _result_3
    (if (`KismetStringLibrary.Contains` (`KismetStringLibrary.Conv_NameToString` _array_element) (`KismetTextLibrary.Conv_TextToString` KeyWords))
      ;;[1 1 1] 添加符合条件的结果
      (`BlueprintSetLibrary.Set_Add` (`self.QueryNames`) (`|GetArrayItem` _result _array_index))
      (`BlueprintSetLibrary.Set_Add` (`self.Query_IDs`) (`|GetArrayItem` _result_2 _array_index))
      (`BlueprintSetLibrary.Set_Add` (`self.Query_RowNames`) _array_element)))
  ;;[1 1 1] 查询完成初始化UI
  (`self.InitQueryDataTableRow` Editor SoftClassPath))

(event `/Game/Resource/BP/Data/ItemIdManager/Property/0Base/BP_ItemID_Edit_PropertyInterface.DataTableLoad`
  (params (Editor :type "/Game/Resource/BP/Data/ItemIdManager/Editor/BP_核心数据表修改器 Object Reference"))
  ;[1 1 1] 将初始化完成的数据，加载显示到编辑器中
  (`self.InitDataTableRow` Editor (`self.Data Table Item Class`)))

(event `/Game/Resource/BP/Data/ItemIdManager/Property/0Base/BP_ItemID_Edit_PropertyInterface.DataTableAdd`
  (params (NewName :type Text) (NewID :type Integer) (Editor :type "/Game/Resource/BP/Data/ItemIdManager/Editor/BP_核心数据表修改器 Object Reference") (DataTable :type "DataTable Object Reference"))
  ;[1 1 1] 新增数据记录
  (`self.AddNewData` (`KismetTextLibrary.Conv_TextToString` NewName) NewID DataTable Editor (`self.Data Table Item Class`)))

(event `/Game/Resource/BP/Data/ItemIdManager/Property/0Base/BP_ItemID_Edit_PropertyInterface.DataTableFindNameByID`
  (params (Editor :type "/Game/Resource/BP/Data/ItemIdManager/Editor/BP_核心数据表修改器 Object Reference") (ItemID :type Integer))
  ;[1 1 1] 查询名称
  (bind _result (`BlueprintSetLibrary.Set_ToArray` (`self.IDs`)))
  (bind _returnvalue (`KismetArrayLibrary.Array_Find` _result ItemID))
  (if (not (== _returnvalue -1))
    (bind _result_2 (`BlueprintSetLibrary.Set_ToArray` (`self.RowNames`)))
    (`/Game/Resource/BP/Data/ItemIdManager/Editor/BP_核心数据表修改器.ShowNameByID` Editor (`KismetTextLibrary.Conv_NameToText` (`|GetArrayItem` _result_2 _returnvalue)))))

(fn `Add`
  (params (RowName :type "Name (by ref)") (ID :type "Integer (by ref)") (Name :type "String (by ref)"))
  (`self.AddRowName` RowName)
  (`self.AddID` ID)
  (`self.AddName` Name))

(fn `AddID`
  (params (ID :type "Integer (by ref)"))
  (`BlueprintSetLibrary.Set_Add` (`self.IDs`) ID))

(fn `AddName`
  (params (Name :type "String (by ref)"))
  (`BlueprintSetLibrary.Set_Add` (`self.Names`) Name))

(fn `AddNewData`
  (params (ItemName :type String) (ItemID :type Integer) (DataTable :type "DataTable Object Reference") (Editor :type "/Game/Resource/BP/Data/ItemIdManager/Editor/BP_核心数据表修改器 Object Reference") (DataTableItemClass :type "SoftClassPath Structure"))
  (`/Game/Resource/BP/Data/ItemIdManager/Editor/BP_核心数据表修改器.CreateItemRowUI` Editor DataTableItemClass ItemName ItemID (`KismetStringLibrary.Conv_StringToName` ItemName)))

(fn `AddNewDataCustom`
  (params (ItemName :type String) (ItemID :type Integer) (DataTable :type "DataTable Object Reference") (Editor :type "/Game/Resource/BP/Data/ItemIdManager/Editor/BP_核心数据表修改器 Object Reference") (DataTableItemClass :type "SoftClassPath Structure"))
  (returns (bResult :type Boolean))
  (`/Game/Resource/BP/Data/ItemIdManager/Editor/BP_核心数据表修改器.CreateItemRowUICustom` Editor DataTableItemClass (`KismetStringLibrary.Conv_StringToName` ItemName) ItemID)
  (return true))

(fn `AddRowName`
  (params (RowName :type "Name (by ref)"))
  (`BlueprintSetLibrary.Set_Add` (`self.RowNames`) RowName))

(fn `DataTableRowFind`
  (params (RowName :type Name))
  (returns (bFind :type Boolean))
  (return false))

(fn `FindRowName`
  (params (RowName :type Name))
  (returns (bFind :type Boolean))
  (return (`BlueprintSetLibrary.Set_Contains` (`self.RowNames`) RowName)))

(fn `GetDataRowName`
  (returns (RowName :type Name))
  (return "None"))

(fn `GetIDs`
  (returns (IDs :type "Set of Integer"))
  (return (`self.IDs`)))

(fn `GetNames`
  (returns (Names :type "Set of String"))
  (return (`self.Names`)))

(fn `GetRowNames`
  (returns (RowNames :type "Set of Name"))
  (return (`self.RowNames`)))

(fn `InitDataTableRow`
  (params (Editor :type "/Game/Resource/BP/Data/ItemIdManager/Editor/BP_核心数据表修改器 Object Reference") (DataTableItemClass :type "SoftClassPath Structure"))
  (`/Game/Resource/BP/Data/ItemIdManager/Editor/BP_核心数据表修改器.InitDataTableRows` Editor (`self.GetIDs`) (`self.GetNames`) (`self.GetRowNames`) DataTableItemClass))

(fn `InitQueryDataTableRow`
  (params (Target :type "/Game/Resource/BP/Data/ItemIdManager/Editor/BP_核心数据表修改器 Object Reference") (DataTableItemClass :type "SoftClassPath Structure"))
  (`/Game/Resource/BP/Data/ItemIdManager/Editor/BP_核心数据表修改器.InitDataTableRows` Target (`self.Query_IDs`) (`self.QueryNames`) (`self.Query_RowNames`) DataTableItemClass))