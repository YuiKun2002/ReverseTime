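; Base Blueprint for custom data table row items in the ItemID editor, handling row addition and name lookup by ID.
; It keeps a running ID counter, reset on table init, which replaces the passed-in ID when adding a row through the parent.
; GetID returns the counter, optionally advancing it.
; The find-name-by-ID override calls the editor's CallSetbListID before deferring to the parent.
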(event `/Game/Resource/BP/Data/ItemIdManager/Property/0Base/BP_ItemID_Edit_PropertyInterface.DataTableInit`
  (params (DataTable :type "DataTable Object Reference"))
  ;[1 1 1] 初始化卡片的数据表数据：添加ID：对应卡片详细数据，添加数据的名称
  (set `self.ID` 0))

(event `/Game/Resource/BP/Data/ItemIdManager/Property/0Base/BP_ItemID_Edit_PropertyInterface.DataTableAdd`
  (params (NewName :type Text) (NewID :type Integer) (Editor :type "/Game/Resource/BP/Data/ItemIdManager/Editor/BP_核心数据表修改器 Object Reference") (DataTable :type "DataTable Object Reference"))
  ;[1 1 1] 重写数据表新增行
  (if (`self.AddNewDataCustom` (`KismetTextLibrary.Conv_TextToString` NewName) NewID DataTable Editor (`self.Data Table Item Class`))
    _))

(event `/Game/Resource/BP/Data/ItemIdManager/Property/0Base/BP_ItemID_Edit_PropertyInterface.DataTableFindNameByID`
  (params (Editor :type "/Game/Resource/BP/Data/ItemIdManager/Editor/BP_核心数据表修改器 Object Reference") (ItemID :type Integer))
  ;[1 1 1] 删除行
  (`/Game/Resource/BP/Data/ItemIdManager/Editor/BP_核心数据表修改器.SetbListID` Editor)
  (`parent.DataTableFindNameByID` Editor ItemID))

(fn `AddNewDataCustom`
  (params (ItemName :type String) (ItemID :type Integer) (DataTable :type "DataTable Object Reference") (Editor :type "/Game/Resource/BP/Data/ItemIdManager/Editor/BP_核心数据表修改器 Object Reference") (DataTableItemClass :type "SoftClassPath Structure"))
  (returns (bResult :type Boolean))
  (bind _result (`/Engine/EditorBlueprintResources/StandardMacros.IncrementInt` (`self.ID`))
    (:`  `
      (return (`parent.AddNewDataCustom` ItemName _result DataTable Editor DataTableItemClass)))))

(fn `GetID`
  (params (`b++` :type Boolean))
  (returns (ID :type Integer))
  (locals (NewLocalVar_0 :type Integer :default 0))
  (if `b++`
    (set `local.NewLocalVar_0` (`self.ID`))
    (`/Engine/EditorBlueprintResources/StandardMacros.IncrementInt` (`self.ID`)
      (:`  `
        (return (`local.NewLocalVar_0`))))
    (else
      (return (`self.ID`)))))