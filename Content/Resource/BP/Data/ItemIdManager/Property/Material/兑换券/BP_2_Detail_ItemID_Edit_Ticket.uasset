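; Detail object for editing exchange-ticket (兑换券) item data in the item ID manager.
; InitDetailClass caches the ticket editor UI widget and copies the entry matching the given Id from the owner's Items map into Data.
; SaveDetail only calls the widget's SaveProperty; the node that would push Data back to the widget is disconnected, despite the comment describing that step.
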(event `/Game/Resource/BP/Data/ItemIdManager/Property/0Base/BP_ItemID_Edit_PropertyInterface.InitDetailClass`
  (params (Owner :type "Object Object Reference") (UI :type "EditorUtilityWidget Object Reference") (Id :type Integer))
  ;[1 1 1] 初始化关联UI项，和初始化物品数据
  (bind _asbp_2_ui_item_id_edit_ticket (cast `/Game/Resource/BP/Data/ItemIdManager/Property/Material/兑换券/BP_2_UI_ItemID_Edit_Ticket` UI))
  (set `self.As BP 2 UI Item ID Edit Ticket` _asbp_2_ui_item_id_edit_ticket)
  (bind _asbp_2_edit_item_id_ticket (cast `/Game/Resource/BP/Data/ItemIdManager/Property/Material/兑换券/BP_2_Edit_ItemID_Ticket` Owner))
  (set `self.Data` (`BlueprintMapLibrary.Map_Find` (`/Game/Resource/BP/Data/ItemIdManager/Property/Material/兑换券/BP_2_Edit_ItemID_Ticket.Items` _asbp_2_edit_item_id_ticket) Id)))

(event `/Game/Resource/BP/Data/ItemIdManager/Property/0Base/BP_ItemID_Edit_PropertyInterface.SaveDetail`
  ;[1 1 1] 当属性发生变化时，自动触发，设置UI项中Data数据，随后让UI进行保存操作
  (`/Game/Resource/BP/Data/ItemIdManager/Property/0Base/BP_ItemID_Edit_PropertyInterface.SaveProperty` (`self.As BP 2 UI Item ID Edit Ticket`)))