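; Detail object for editing one entry of the gold card evolution match table in the ItemID manager.
; InitDetailClass casts and caches the list UI item, then loads the entry's Data from the owning editor's Items map by Id.
; SaveDetail, noted as firing automatically on property changes, copies Data back into the UI item and calls its SaveProperty to save.
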(event `/Game/Resource/BP/Data/ItemIdManager/Property/0Base/BP_ItemID_Edit_PropertyInterface.InitDetailClass`
  (params (Owner :type "Object Object Reference") (UI :type "EditorUtilityWidget Object Reference") (Id :type Integer))
  ;[1 1 1] 初始化关联UI项，和初始化物品数据
  (bind _asbp__2_ui_item_id_edit_gold_card_up_data (cast `/Game/Resource/BP/Data/ItemIdManager/Property/Material/其他特殊表格/金卡进化匹配表/BP_-2_UI_ItemID_Edit_GoldCardUpData` UI))
  (set `self.As BP -2 UI Item ID Edit Gold Card Up Data` _asbp__2_ui_item_id_edit_gold_card_up_data)
  (bind _asbp__2_edit_item_id_gold_card_up_data (cast `/Game/Resource/BP/Data/ItemIdManager/Property/Material/其他特殊表格/金卡进化匹配表/BP_-2_Edit_ItemID_GoldCardUpData` Owner))
  (set `self.Data` (`BlueprintMapLibrary.Map_Find` (`/Game/Resource/BP/Data/ItemIdManager/Property/Material/其他特殊表格/金卡进化匹配表/BP_-2_Edit_ItemID_GoldCardUpData.Items` _asbp__2_edit_item_id_gold_card_up_data) Id)))

(event `/Game/Resource/BP/Data/ItemIdManager/Property/0Base/BP_ItemID_Edit_PropertyInterface.SaveDetail`
  (bind _as_bp__2_ui_item_id_edit_gold_card_up_data (`self.As BP -2 UI Item ID Edit Gold Card Up Data`))
  ;[1 1 1] 当属性发生变化时，自动触发，设置UI项中Data数据，随后让UI进行保存操作
  (set `/Game/Resource/BP/Data/ItemIdManager/Property/Material/其他特殊表格/金卡进化匹配表/BP_-2_UI_ItemID_Edit_GoldCardUpData.Data` (`self.Data`) _as_bp__2_ui_item_id_edit_gold_card_up_data)
  (`/Game/Resource/BP/Data/ItemIdManager/Property/0Base/BP_ItemID_Edit_PropertyInterface.SaveProperty` _as_bp__2_ui_item_id_edit_gold_card_up_data))