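; Item ID data Blueprint for the gold card evolution matching table, which loads a data table into ID-keyed entries.
; It overrides DataTableInit, calls the parent, then walks every row name and stores each found row in Items under a generated ID.
; Each row name is also registered with its ID and display name, and a completion message prints at the end.
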(event `/Game/Resource/BP/Data/ItemIdManager/Property/0Base/BP_ItemID_Edit_PropertyInterface.DataTableInit`
  (params (DataTable :type "DataTable Object Reference"))
  ;[1 1 1] 初始化卡片的数据表数据：添加ID：对应卡片详细数据，添加数据的名称
  (`parent.DataTableInit` DataTable)
  (bind _outrownames (`DataTableFunctionLibrary.GetDataTableRowNames` DataTable))
  (for _array_element _outrownames
    (bind _returnvalue (`|GetDataTableRow` DataTable _array_element)
      (:`then`
        (`BlueprintMapLibrary.Map_Add` (`self.Items`) (`self.GetID` false) _returnvalue)
        (`self.Add` _array_element (`self.GetID` true) (`KismetStringLibrary.Conv_NameToString` _array_element)))))
  (`KismetSystemLibrary.PrintString` null "数据初始化完成"))