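; Detail object for editing one entry of the defense card skill book matching table in the ItemID data editor.
; InitDetailClass caches the linked UI item and copies the entry for the given Id from the owning editor's Items map into Data.
; SaveDetail, noted as firing automatically on property changes, pushes Data back to the UI item and calls its SaveProperty to save.
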(event `/Game/Resource/BP/Data/ItemIdManager/Property/0Base/BP_ItemID_Edit_PropertyInterface.InitDetailClass`
  (params (Owner :type "Object Object Reference") (UI :type "EditorUtilityWidget Object Reference") (Id :type Integer))
  ;[1 1 1] 初始化关联UI项，和初始化物品数据
  (bind _asbp__2_ui_item_id_edit_card_skillbooks_data (cast `/Game/Resource/BP/Data/ItemIdManager/Property/Material/其他特殊表格/防御卡技能书匹配表/BP_-2_UI_ItemID_Edit_CardSkillbooksData` UI))
  (set `self.As BP -2 UI Item ID Edit Card Skillbooks Data` _asbp__2_ui_item_id_edit_card_skillbooks_data)
  (bind _asbp__2_edit_item_id_card_skillbooks_data (cast `/Game/Resource/BP/Data/ItemIdManager/Property/Material/其他特殊表格/防御卡技能书匹配表/BP_-2_Edit_ItemID_CardSkillbooksData` Owner))
  (set `self.Data` (`BlueprintMapLibrary.Map_Find` (`/Game/Resource/BP/Data/ItemIdManager/Property/Material/其他特殊表格/防御卡技能书匹配表/BP_-2_Edit_ItemID_CardSkillbooksData.Items` _asbp__2_edit_item_id_card_skillbooks_data) Id)))

(event `/Game/Resource/BP/Data/ItemIdManager/Property/0Base/BP_ItemID_Edit_PropertyInterface.SaveDetail`
  (bind _as_bp__2_ui_item_id_edit_card_skillbooks_data (`self.As BP -2 UI Item ID Edit Card Skillbooks Data`))
  ;[1 1 1] 当属性发生变化时，自动触发，设置UI项中Data数据，随后让UI进行保存操作
  (set `/Game/Resource/BP/Data/ItemIdManager/Property/Material/其他特殊表格/防御卡技能书匹配表/BP_-2_UI_ItemID_Edit_CardSkillbooksData.Data` (`self.Data`) _as_bp__2_ui_item_id_edit_card_skillbooks_data)
  (`/Game/Resource/BP/Data/ItemIdManager/Property/0Base/BP_ItemID_Edit_PropertyInterface.SaveProperty` _as_bp__2_ui_item_id_edit_card_skillbooks_data))