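; Detail object for editing one drill bit entry's data in the item ID manager.
; InitDetailClass casts and caches the linked UI item, then copies the entry's Data from the owning BP_2_Edit_ItemID_Bit's Items map by Id.
; SaveDetail, noted as firing automatically on property changes, pushes Data back into the UI item and calls its SaveProperty, leaving persistence to that widget.
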(event `/Game/Resource/BP/Data/ItemIdManager/Property/0Base/BP_ItemID_Edit_PropertyInterface.InitDetailClass`
  (params (Owner :type "Object Object Reference") (UI :type "EditorUtilityWidget Object Reference") (Id :type Integer))
  ;[1 1 1] 初始化关联UI项，和初始化物品数据
  (bind _asbp_2_ui_item_id_edit_bit (cast `/Game/Resource/BP/Data/ItemIdManager/Property/Material/钻头/BP_2_UI_ItemID_Edit_Bit` UI))
  (set `self.As BP 2 UI Item ID Edit Bit` _asbp_2_ui_item_id_edit_bit)
  (bind _asbp_2_edit_item_id_bit (cast `/Game/Resource/BP/Data/ItemIdManager/Property/Material/钻头/BP_2_Edit_ItemID_Bit` Owner))
  (set `self.Data` (`BlueprintMapLibrary.Map_Find` (`/Game/Resource/BP/Data/ItemIdManager/Property/Material/钻头/BP_2_Edit_ItemID_Bit.Items` _asbp_2_edit_item_id_bit) Id)))

(event `/Game/Resource/BP/Data/ItemIdManager/Property/0Base/BP_ItemID_Edit_PropertyInterface.SaveDetail`
  (bind _as_bp_2_ui_item_id_edit_bit (`self.As BP 2 UI Item ID Edit Bit`))
  ;[1 1 1] 当属性发生变化时，自动触发，设置UI项中Data数据，随后让UI进行保存操作
  (set `/Game/Resource/BP/Data/ItemIdManager/Property/Material/钻头/BP_2_UI_ItemID_Edit_Bit.Data` (`self.Data`) _as_bp_2_ui_item_id_edit_bit)
  (`/Game/Resource/BP/Data/ItemIdManager/Property/0Base/BP_ItemID_Edit_PropertyInterface.SaveProperty` _as_bp_2_ui_item_id_edit_bit))