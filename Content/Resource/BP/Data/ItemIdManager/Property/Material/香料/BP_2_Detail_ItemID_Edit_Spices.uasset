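; Detail object for editing one spice material entry in the item ID manager.
; On init it casts and caches the spices UI item, then loads that ID's data from the owning spices edit object's Items map.
; When a property changes, SaveDetail copies the edited Data back into the UI item and calls its SaveProperty to save it.
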(event `/Game/Resource/BP/Data/ItemIdManager/Property/0Base/BP_ItemID_Edit_PropertyInterface.InitDetailClass`
  (params (Owner :type "Object Object Reference") (UI :type "EditorUtilityWidget Object Reference") (Id :type Integer))
  ;[1 1 1] 初始化关联UI项，和初始化物品数据
  (bind _asbp_2_ui_item_id_edit_spices (cast `/Game/Resource/BP/Data/ItemIdManager/Property/Material/香料/BP_2_UI_ItemID_Edit_Spices` UI))
  (set `self.As BP 2 UI Item ID Edit Spices` _asbp_2_ui_item_id_edit_spices)
  (bind _asbp_2_edit_item_id_spices (cast `/Game/Resource/BP/Data/ItemIdManager/Property/Material/香料/BP_2_Edit_ItemID_Spices` Owner))
  (set `self.Data` (`BlueprintMapLibrary.Map_Find` (`/Game/Resource/BP/Data/ItemIdManager/Property/Material/香料/BP_2_Edit_ItemID_Spices.Items` _asbp_2_edit_item_id_spices) Id)))

(event `/Game/Resource/BP/Data/ItemIdManager/Property/0Base/BP_ItemID_Edit_PropertyInterface.SaveDetail`
  (bind _as_bp_2_ui_item_id_edit_spices (`self.As BP 2 UI Item ID Edit Spices`))
  ;[1 1 1] 当属性发生变化时，自动触发，设置UI项中Data数据，随后让UI进行保存操作
  (set `/Game/Resource/BP/Data/ItemIdManager/Property/Material/香料/BP_2_UI_ItemID_Edit_Spices.Data` (`self.Data`) _as_bp_2_ui_item_id_edit_spices)
  (`/Game/Resource/BP/Data/ItemIdManager/Property/0Base/BP_ItemID_Edit_PropertyInterface.SaveProperty` _as_bp_2_ui_item_id_edit_spices))