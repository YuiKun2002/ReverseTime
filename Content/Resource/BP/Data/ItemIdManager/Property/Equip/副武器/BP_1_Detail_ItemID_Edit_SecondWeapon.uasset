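; Detail object for editing one secondary weapon entry in the item ID editor.
; InitDetailClass caches the linked secondary weapon UI widget and loads Data from the owning editor's Items map by ID, stopping if a cast fails.
; SaveDetail, noted as firing automatically on property changes, copies the edited Data into that widget and calls its SaveProperty to handle saving.
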(event `/Game/Resource/BP/Data/ItemIdManager/Property/0Base/BP_ItemID_Edit_PropertyInterface.InitDetailClass`
  (params (Owner :type "Object Object Reference") (UI :type "EditorUtilityWidget Object Reference") (Id :type Integer))
  ;[1 1 1] 初始化关联UI项，和初始化物品数据
  (bind _asbp_1_ui_item_id_edit_second_weapon (cast `/Game/Resource/BP/Data/ItemIdManager/Property/Equip/副武器/BP_1_UI_ItemID_Edit_SecondWeapon` UI))
  (set `self.As BP 1 UI Item ID Edit Second Weapon` _asbp_1_ui_item_id_edit_second_weapon)
  (bind _asbp_1_edit_item_id_second_weapon (cast `/Game/Resource/BP/Data/ItemIdManager/Property/Equip/副武器/BP_1_Edit_ItemID_SecondWeapon` Owner))
  (set `self.Data` (`BlueprintMapLibrary.Map_Find` (`/Game/Resource/BP/Data/ItemIdManager/Property/Equip/副武器/BP_1_Edit_ItemID_SecondWeapon.Items` _asbp_1_edit_item_id_second_weapon) Id)))

(event `/Game/Resource/BP/Data/ItemIdManager/Property/0Base/BP_ItemID_Edit_PropertyInterface.SaveDetail`
  (bind _as_bp_1_ui_item_id_edit_second_weapon (`self.As BP 1 UI Item ID Edit Second Weapon`))
  ;[1 1 1] 当属性发生变化时，自动触发，设置UI项中Data数据，随后让UI进行保存操作
  (set `/Game/Resource/BP/Data/ItemIdManager/Property/Equip/副武器/BP_1_UI_ItemID_Edit_SecondWeapon.Data` (`self.Data`) _as_bp_1_ui_item_id_edit_second_weapon)
  (`/Game/Resource/BP/Data/ItemIdManager/Property/0Base/BP_ItemID_Edit_PropertyInterface.SaveProperty` _as_bp_1_ui_item_id_edit_second_weapon))