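; Detail object for editing a super weapon entry in the item ID manager, under the equipment property data.
; InitDetailClass casts and caches the linked super weapon UI item, then loads Data from the owning editor's Items map by Id.
; SaveDetail, noted as firing automatically on property changes, copies Data back to that UI item and calls its SaveProperty to save it.
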(event `/Game/Resource/BP/Data/ItemIdManager/Property/0Base/BP_ItemID_Edit_PropertyInterface.InitDetailClass`
  (params (Owner :type "Object Object Reference") (UI :type "EditorUtilityWidget Object Reference") (Id :type Integer))
  ;[1 1 1] 初始化关联UI项，和初始化物品数据
  (bind _asbp_1_ui_item_id_edit_super_weapon (cast `/Game/Resource/BP/Data/ItemIdManager/Property/Equip/超级武器/BP_1_UI_ItemID_Edit_SuperWeapon` UI))
  (set `self.As BP 1 UI Item ID Edit Super Weapon` _asbp_1_ui_item_id_edit_super_weapon)
  (bind _asbp_1_edit_item_id_super_weapon (cast `/Game/Resource/BP/Data/ItemIdManager/Property/Equip/超级武器/BP_1_Edit_ItemID_SuperWeapon` Owner))
  (set `self.Data` (`BlueprintMapLibrary.Map_Find` (`/Game/Resource/BP/Data/ItemIdManager/Property/Equip/超级武器/BP_1_Edit_ItemID_SuperWeapon.Items` _asbp_1_edit_item_id_super_weapon) Id)))

(event `/Game/Resource/BP/Data/ItemIdManager/Property/0Base/BP_ItemID_Edit_PropertyInterface.SaveDetail`
  (bind _as_bp_1_ui_item_id_edit_super_weapon (`self.As BP 1 UI Item ID Edit Super Weapon`))
  ;[1 1 1] 当属性发生变化时，自动触发，设置UI项中Data数据，随后让UI进行保存操作
  (set `/Game/Resource/BP/Data/ItemIdManager/Property/Equip/超级武器/BP_1_UI_ItemID_Edit_SuperWeapon.Data` (`self.Data`) _as_bp_1_ui_item_id_edit_super_weapon)
  (`/Game/Resource/BP/Data/ItemIdManager/Property/0Base/BP_ItemID_Edit_PropertyInterface.SaveProperty` _as_bp_1_ui_item_id_edit_super_weapon))