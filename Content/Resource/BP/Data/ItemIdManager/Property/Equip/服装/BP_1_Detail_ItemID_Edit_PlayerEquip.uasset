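; Detail object for editing one player-equipment (clothing) entry in the ItemID data editor.
; InitDetailClass caches the equipment UI entry and loads Data from the owning editor's Items map by Id.
; When a property changes, SaveDetail copies Data into that UI entry and calls its SaveProperty, leaving persistence to the UI.
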(event `/Game/Resource/BP/Data/ItemIdManager/Property/0Base/BP_ItemID_Edit_PropertyInterface.InitDetailClass`
  (params (Owner :type "Object Object Reference") (UI :type "EditorUtilityWidget Object Reference") (Id :type Integer))
  ;[1 1 1] 初始化关联UI项，和初始化物品数据
  (bind _asbp_1_ui_item_id_edit_player_equip (cast `/Game/Resource/BP/Data/ItemIdManager/Property/Equip/服装/BP_1_UI_ItemID_Edit_PlayerEquip` UI))
  (set `self.As BP 1 UI Item ID Edit Player Equip` _asbp_1_ui_item_id_edit_player_equip)
  (bind _asbp_1_edit_item_id_player_equip (cast `/Game/Resource/BP/Data/ItemIdManager/Property/Equip/服装/BP_1_Edit_ItemID_PlayerEquip` Owner))
  (set `self.Data` (`BlueprintMapLibrary.Map_Find` (`/Game/Resource/BP/Data/ItemIdManager/Property/Equip/服装/BP_1_Edit_ItemID_PlayerEquip.Items` _asbp_1_edit_item_id_player_equip) Id)))

(event `/Game/Resource/BP/Data/ItemIdManager/Property/0Base/BP_ItemID_Edit_PropertyInterface.SaveDetail`
  (bind _as_bp_1_ui_item_id_edit_player_equip (`self.As BP 1 UI Item ID Edit Player Equip`))
  ;[1 1 1] 当属性发生变化时，自动触发，设置UI项中Data数据，随后让UI进行保存操作
  (set `/Game/Resource/BP/Data/ItemIdManager/Property/Equip/服装/BP_1_UI_ItemID_Edit_PlayerEquip.Data` (`self.Data`) _as_bp_1_ui_item_id_edit_player_equip)
  (`/Game/Resource/BP/Data/ItemIdManager/Property/0Base/BP_ItemID_Edit_PropertyInterface.SaveProperty` _as_bp_1_ui_item_id_edit_player_equip))