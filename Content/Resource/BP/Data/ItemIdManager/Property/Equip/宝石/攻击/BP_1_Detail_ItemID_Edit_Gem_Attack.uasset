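; Detail object for editing one attack gem entry in the item ID manager, bridging its property data and the editor UI.
; InitDetailClass caches the matching UI item and copies the entry for the given Id from the owner's Items map into Dara.
; SaveDetail, noted as firing automatically on property changes, pushes Dara back to that UI item and calls its SaveProperty to handle saving.
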(event `/Game/Resource/BP/Data/ItemIdManager/Property/0Base/BP_ItemID_Edit_PropertyInterface.InitDetailClass`
  (params (Owner :type "Object Object Reference") (UI :type "EditorUtilityWidget Object Reference") (Id :type Integer))
  ;[1 1 1] 初始化关联UI项，和初始化物品数据
  (bind _asbp_1_ui_item_id_edit_gem_attack (cast `/Game/Resource/BP/Data/ItemIdManager/Property/Equip/宝石/攻击/BP_1_UI_ItemID_Edit_Gem_Attack` UI))
  (set `self.As BP 1 UI Item ID Edit Gem Attack_0` _asbp_1_ui_item_id_edit_gem_attack)
  (bind _asbp_1_edit_item_id_gem_attack (cast `/Game/Resource/BP/Data/ItemIdManager/Property/Equip/宝石/攻击/BP_1_Edit_ItemID_Gem_Attack` Owner))
  (set `self.Dara` (`BlueprintMapLibrary.Map_Find` (`/Game/Resource/BP/Data/ItemIdManager/Property/Equip/宝石/攻击/BP_1_Edit_ItemID_Gem_Attack.Items` _asbp_1_edit_item_id_gem_attack) Id)))

(event `/Game/Resource/BP/Data/ItemIdManager/Property/0Base/BP_ItemID_Edit_PropertyInterface.SaveDetail`
  (bind _as_bp_1_ui_item_id_edit_gem_attack_0 (`self.As BP 1 UI Item ID Edit Gem Attack_0`))
  ;[1 1 1] 当属性发生变化时，自动触发，设置UI项中Data数据，随后让UI进行保存操作
  (set `/Game/Resource/BP/Data/ItemIdManager/Property/Equip/宝石/攻击/BP_1_UI_ItemID_Edit_Gem_Attack.Dara` (`self.Dara`) _as_bp_1_ui_item_id_edit_gem_attack_0)
  (`/Game/Resource/BP/Data/ItemIdManager/Property/0Base/BP_ItemID_Edit_PropertyInterface.SaveProperty` _as_bp_1_ui_item_id_edit_gem_attack_0))