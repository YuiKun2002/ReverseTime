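; BP_APlayerView is a player view Blueprint with a camera component, kept with the GameStart game mode assets.
; Its graphs hold only disconnected logic, so none of it executes.
; The unused event logic toggles game pause unless the game is over, showing the BP_GamePause widget when pausing.
; The construction script is empty, beside unwired nodes that would make the camera orthographic.
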(event `Key|BackSpace`
  (params (Key :type "Key Structure")))

(event `Key|SpaceBar`
  (params (Key :type "Key Structure")))

(event `Key|Escape`
  (params (Key :type "Key Structure")))

(fn `UserConstructionScript`)