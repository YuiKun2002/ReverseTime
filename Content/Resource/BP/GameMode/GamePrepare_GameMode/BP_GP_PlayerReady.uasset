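; Per-player networked actor for the game-preparation lobby, handling joining, ready toggling and game start.
; The client loads saved name, gender and suit, joins through the GameMode, then updates the prepare UI.
; The server toggles the player's ID in GameState's ReadyID and multicasts the array so clients refresh at once.
; Game start async-loads the level behind a fullscreen widget, then runs a ServerTravel console command after a delay.
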(event `Client_ReadPlayerLocalData`
  (params (PlayerID :type String))
  (bind _returnvalue (`FVMGameInstance.GetFVMGameInstance`))
  ;[1 1 1] 从本地客户端加载本地数据，更新到角色信息，请求服务器加入游戏
  (cast `/Game/Resource/BP/GameMode/GamePrepare_GameMode/BP_GP_PC` (`self.GetController`))
  (bind _returnvalue_2 (`FVMGameInstance.LoadPlayerStructManager` _returnvalue (`FVMGameInstance.GetPlayerLoginName` _returnvalue)))
  (`self.Server_Join` (make `/Game/Resource/BP/GameMode/GamePrepare_GameMode/BP_GamePrepare_PlayerInfor` :`Name` (`PlayerStructManager.M_PlayerName` _returnvalue_2) :`Gender` (`PlayerStructManager.M_PlayerGender` _returnvalue_2) :`Suit` (`PlayerStructManager.M_FPlayerSuit` _returnvalue_2) :`PlayerID` PlayerID)))

(event `Server_Join`
  (params (PlayerInfor :type "/Game/Resource/BP/GameMode/GamePrepare_GameMode/BP_GamePrepare_PlayerInfor Structure"))
  ;[1 1 1] 从本地客户端加载本地数据，更新到角色信息，请求服务器加入游戏
  ;;[1 1 1] 请求服务器
  (bind _asbp_game_prepare_game_mode (cast `/Game/Resource/BP/GameMode/GamePrepare_GameMode/BP_GamePrepare_GameMode` (`GameplayStatics.GetGameMode`)))
  (`/Game/Resource/BP/GameMode/GamePrepare_GameMode/BP_GamePrepare_GameMode.Server_Join` _asbp_game_prepare_game_mode PlayerInfor))

(event `Client_UpdateGameReadyWidget`
  (params (PC :type "/Game/Resource/BP/GameMode/GamePrepare_GameMode/BP_GP_PC Object Reference") (PlayerInfor :type "Array of /Game/Resource/BP/GameMode/GamePrepare_GameMode/BP_GamePrepare_PlayerInfor Structure"))
  (bind _returnvalue (`GameUserInterfaceInstance.GetUI` (`GameSystemFunction.GetUserInterInstanceByClass` "/Game/Resource/BP/Data/GameData/CategoryName/UIName/CategoryName_UI_Global/BP_CategoryName_UI_Global.BP_CategoryName_UI_Global_C") (`GameDataName.Get_UI_GamePrepare`)))
  ;[1 1 1] 准备UI界面-完成登陆-进行UI更新
  (`UserWidget.SetOwningPlayer` _returnvalue PC)
  (if (`Widget.IsInViewport` _returnvalue)
    (bind _asbpui_game_prepare (cast `/Game/Resource/BP/Game/UI/GamePrepare/BPUI_GamePrepare` _returnvalue))
    (`/Game/Resource/BP/Game/UI/GamePrepare/BPUI_GamePrepare.GameReady` _asbpui_game_prepare PlayerInfor)
    (else
      (bind _asbpui_game_prepare_2 (cast `/Game/Resource/BP/Game/UI/GamePrepare/BPUI_GamePrepare` _returnvalue))
      (`/Game/Resource/BP/Game/UI/GamePrepare/BPUI_GamePrepare.GameReady` _asbpui_game_prepare_2 PlayerInfor)
      (`UserWidget.AddToViewport` _asbpui_game_prepare_2 0)
      (`FVMGameInstance.PlayBGM_Static` (`KismetSystemLibrary.MakeSoftObjectPath` (`self.BgmStr`)))))
  (if (`FVMGameInstance.GetDebug`)
    (`GameUserInterfaceInstance.ShowUI_ByName` (`GameSystemFunction.GetUserInterInstanceByClass` "/Game/Resource/BP/Data/GameData/CategoryName/UIName/CategoryName_UI_Global/BP_CategoryName_UI_Global.BP_CategoryName_UI_Global_C") (`GameDataName.Get_UI_GameTest`) 1)))

(event `Client_GameStart`
  ;[1 1 1] 游戏开始
  (`|LoadAsset` "/Game/Resource/Level/Online/BP_GameStartLevel.BP_GameStartLevel"
    (:`then`
      (bind _returnvalue (`|CreateWidget` "/Game/Resource/BP/GameStart/VS/UI_Player/UICardBad/FullScreen.FullScreen_C"))
      (`UserWidget.AddToViewport` _returnvalue 0))
    (:`Completed`
      (`KismetSystemLibrary.Delay` 1.0)
      (`KismetSystemLibrary.ExecuteConsoleCommand` "ServerTravel BP_GameStartLevel" (`GameplayStatics.GetPlayerController` 0)))))

(event `Server_GameReady`
  ;[1 1 1] 玩家准备操作
  ;;[1 1 1] 玩家准备或者取消准备
  (bind _asbp_gp_pc (cast `/Game/Resource/BP/GameMode/GamePrepare_GameMode/BP_GP_PC` (`self.GetController`)))
  (bind _asbp_game_prepare_gs (cast `/Game/Resource/BP/GameMode/GamePrepare_GameMode/BP_GamePrepare_GS` (`GameplayStatics.GetGameState`)))
  (bind _playerid (`/Game/Resource/BP/GameMode/GamePrepare_GameMode/BP_GP_PC.PlayerID` _asbp_gp_pc))
  (bind _returnvalue (`KismetArrayLibrary.Array_Find` (`/Game/Resource/BP/GameMode/GamePrepare_GameMode/BP_GamePrepare_GS.ReadyID` _asbp_game_prepare_gs) _playerid))
  (if (!= _returnvalue -1)
    (bind _readyid (`/Game/Resource/BP/GameMode/GamePrepare_GameMode/BP_GamePrepare_GS.ReadyID` _asbp_game_prepare_gs))
    (`KismetArrayLibrary.Array_Remove` _readyid _returnvalue)
    (else
      (`KismetArrayLibrary.Array_Add` _readyid _playerid)))
  (`self.Multi_GameReady` (`/Game/Resource/BP/GameMode/GamePrepare_GameMode/BP_GamePrepare_GS.ReadyID` _asbp_game_prepare_gs)) ; 在服务器设置完毕后，立刻进行广播修改的数据\n防止客户端拿不到最新数据
)

(event `Multi_GameReady`
  (params (Readys :type "Array of String"))
  (bind _returnvalue (`GameUserInterfaceInstance.GetUI` (`GameSystemFunction.GetUserInterInstanceByClass` "/Game/Resource/BP/Data/GameData/CategoryName/UIName/CategoryName_UI_Global/BP_CategoryName_UI_Global.BP_CategoryName_UI_Global_C") (`GameDataName.Get_UI_GamePrepare`)))
  ;[1 1 1] 玩家准备操作
  ;;[1 1 1] 让所有的客户端，同步设置
  (bind _asbp_game_prepare_gs (cast `/Game/Resource/BP/GameMode/GamePrepare_GameMode/BP_GamePrepare_GS` (`GameplayStatics.GetGameState`))) ; 让本地客户端立刻刷新被设置的数据\n不会因为延迟，丢包等情况出现数据不同步的情况
  (set `/Game/Resource/BP/GameMode/GamePrepare_GameMode/BP_GamePrepare_GS.ReadyID` Readys _asbp_game_prepare_gs)
  (if (`Widget.IsInViewport` _returnvalue)
    (bind _asbpui_game_prepare (cast `/Game/Resource/BP/Game/UI/GamePrepare/BPUI_GamePrepare` _returnvalue))
    (`/Game/Resource/BP/Game/UI/GamePrepare/BPUI_GamePrepare.Init Ready Game` _asbpui_game_prepare true)))

(event `Server_UpdateReady`
  (params (Readys :type "Array of String (by ref)"))
  ;[1 1 1] 玩家准备操作
  ;;[1 1 1] 更新玩家的准备情况
  (`self.Multi_GameReady` Readys))

(fn `UserConstructionScript`)