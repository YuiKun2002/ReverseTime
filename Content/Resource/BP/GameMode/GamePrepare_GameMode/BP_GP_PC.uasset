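; Player controller for the game-preparation stage, handling session updates, joining and leaving.
; A server event skips player IDs the game mode already has, otherwise tells the possessed ready pawn to load client-local data, retrying after a short delay until possession succeeds.
; A client event updates the online session with room info.
; Logout destroys the session and opens a level, with the host first clearing the game mode's player list.
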(event `Client_UpdateRoomInfor`
  (params (Genders :type "Array of Byte"))
  ;[1 1 1] 更新会话信息
  (bind _returnvalue (`MultiplayerOnlineObject.MakeMultiplayerOnlineObject`))
  (`MultiplayerOnlineObject.UpdateOnlineSession` _returnvalue Genders))

(event `Server_ControllerPawn`
  (params (PlayerID :type String))
  (bind _returnvalue (`self.K2_GetPawn`))
  ;[1 1 1] 检测角色控制器控制情况，控制成功则加入游戏
  (bind _asbp_game_prepare_game_mode (cast `/Game/Resource/BP/GameMode/GamePrepare_GameMode/BP_GamePrepare_GameMode` (`GameplayStatics.GetGameMode`))
    (:`then`
      (bind _result (`/Game/Resource/BP/GameMode/GamePrepare_GameMode/BP_GamePrepare_GameMode.CheckHasPlayer` _asbp_game_prepare_game_mode PlayerID))
      (if _result
        (`KismetSystemLibrary.PrintString` "当前玩家已经存在，忽略本次检测")
        (else
          (`/Engine/EditorBlueprintResources/StandardMacros.IsValid` _returnvalue
            (:`Is Valid`
              (bind _asbp_gp_player_ready (cast `/Game/Resource/BP/GameMode/GamePrepare_GameMode/BP_GP_PlayerReady` _returnvalue)
                (:`then`
                  (`/Game/Resource/BP/GameMode/GamePrepare_GameMode/BP_GP_PlayerReady.Client_ReadPlayerLocalData` _asbp_gp_player_ready PlayerID) ; 让此客户端加载自己的本地数据
                )
                (:`CastFailed`
                  (`self.Server_ReControllerPawn` PlayerID))))
            (:`Is Not Valid`
              (`self.Server_ReControllerPawn` PlayerID))))))
    (:`CastFailed`
      (`KismetSystemLibrary.PrintString` "游戏模式 无效"))))

(event `Server_ReControllerPawn`
  (params (PlayerID :type String))
  ;[1 1 1] 控制器没有控制对象，重新进行控制
  (`KismetSystemLibrary.Delay` 0.2)
  (`KismetSystemLibrary.PrintString` "重新进行控制器控制检测")
  (`self.Server_ControllerPawn` PlayerID))

(event `Client_Logout`
  ;[1 1 1] 退出游戏
  (if (or (`KismetSystemLibrary.IsServer`) (`KismetSystemLibrary.IsDedicatedServer`))
    (`/Engine/EditorBlueprintResources/ActorMacros.Switch Has Authority`
      (:`Authority`
        (if (`FVMGameInstance.IsServer` (`FVMGameInstance.GetFVMGameInstance`))
          (bind _asbp_game_prepare_game_mode (cast `/Game/Resource/BP/GameMode/GamePrepare_GameMode/BP_GamePrepare_GameMode` (`GameplayStatics.GetGameMode`)))
          (`KismetArrayLibrary.Array_Clear` (`/Game/Resource/BP/GameMode/GamePrepare_GameMode/BP_GamePrepare_GameMode.PlayerIDList` _asbp_game_prepare_game_mode))))
      (:`Remote`
        _)))
  (`DestroySessionCallbackProxy.DestroySession` self
    (:`then`
      (`KismetSystemLibrary.PrintString` (`KismetStringLibrary.Concat_StrStr` (`self.PlayerID`) "【准备离开游戏】")))
    (:`OnSuccess`
      (`GameplayStatics.OpenLevel` "Game"))
    (:`OnFailure`
      (`GameplayStatics.OpenLevel` "Open"))))

(fn `UserConstructionScript`)