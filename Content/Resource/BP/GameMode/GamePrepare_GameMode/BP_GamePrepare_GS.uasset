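; BP_GamePrepare_GS is the GamePrepare mode's game state, holding basic room info for the preparation room the host enters.
; On BeginPlay it acts only when running as a server or dedicated server and the FVM game instance also reports server.
; It then loads the cached room-creation data and copies the room name, level config and that config's level name as the map name.
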(event `self.ReceiveBeginPlay`
  ;[1 1 1] 房主进入准备房间，更新房间的基本信息
  (if (or (`KismetSystemLibrary.IsServer`) (`KismetSystemLibrary.IsDedicatedServer`))
    (if (`FVMGameInstance.IsServer` (`FVMGameInstance.GetFVMGameInstance`))
      (bind _cache (`/Game/Resource/BP/Game/UI/RoomCreate/BP_PlayerCreateRoomInforFunc.Load Create Room Cache`))
      (set `self.RoomName` (`/Game/Resource/BP/Game/UI/RoomCreate/BP_PlayerCreateRoomInfor.RoomName` _cache))
      (bind _levelconfig (`/Game/Resource/BP/Game/UI/RoomCreate/BP_PlayerCreateRoomInfor.LevelConfig` _cache))
      (set `self.LevelConfig` _levelconfig)
      (set `self.MapName` (`.LevelName` (break `LevelConfig` _levelconfig))))))

(fn `UserConstructionScript`)