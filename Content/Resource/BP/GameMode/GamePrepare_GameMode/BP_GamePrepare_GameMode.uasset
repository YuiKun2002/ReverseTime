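; Game mode for the pre-game room, managing player admission, the roster, readiness checks and game start.
; PostLogin builds an ID from timestamp and controller name, then holds players in TempList or logs them out if the room is full.
; Joining moves them to PlayerIDList, whose first entry becomes owner; joins and non-owner departures refresh clients' UI.
; Start requires the GameState's ready count to equal players minus one, then notifies every player's pawn.
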(event `Server_PlayerLogin`
  (params (NewPlayer :type "/Game/Resource/BP/GameMode/GamePrepare_GameMode/BP_GamePrepare_PlayerInfor Structure"))
  ;[1 1 1] 玩家加入
  (bind (_playerinfor _result) (`self.Check Player` NewPlayer))
  (if _result
    (bind ((`PlayerController_14_0CFF2C2243D3BB09CA066A88EA0952CA` _playercontroller) (`PlayerID_17_82A6292246D93206D86F94827F3246E7` _playerid)) (break `/Game/Resource/BP/GameMode/GamePrepare_GameMode/BP_GamePrepare_PlayerInfor` _playerinfor))
    (bind _output_get (set `/Game/Resource/BP/GameMode/GamePrepare_GameMode/BP_GP_PC.PlayerID` _playerid _playercontroller))
    (`KismetArrayLibrary.Array_Add` (`self.TempList`) _playerinfor)
    (`/Game/Resource/BP/GameMode/GamePrepare_GameMode/BP_GP_PC.Server_ControllerPawn` _playercontroller _output_get)
    (else
      (`self.JoinFailed` NewPlayer))))

(event `Server_Join`
  (params (PlayerInfor :type "/Game/Resource/BP/GameMode/GamePrepare_GameMode/BP_GamePrepare_PlayerInfor Structure"))
  ;[1 1 1] 加入游戏，更新UI界面，更新服务器会话信息
  (bind _result (`self.MoveTempPlayerInfor` PlayerInfor))
  (if _result
    (bind _asbp_game_prepare_gs (cast `/Game/Resource/BP/GameMode/GamePrepare_GameMode/BP_GamePrepare_GS` (`GameplayStatics.GetGameState`)))
    (set `/Game/Resource/BP/GameMode/GamePrepare_GameMode/BP_GamePrepare_GS.RoomOwnerID` (`.PlayerID_17_82A6292246D93206D86F94827F3246E7` (break `/Game/Resource/BP/GameMode/GamePrepare_GameMode/BP_GamePrepare_PlayerInfor` (`|GetArrayItem` (`self.PlayerIDList`)))) _asbp_game_prepare_gs)
    (`KismetSystemLibrary.PrintString` "加入")
    (`self.Server_UpdateAllPlayer`)
    (else
      (`KismetSystemLibrary.PrintString` "没有此玩家"))))

(event `Server_UpdateAllPlayer`
  (bind _playeridlist (`self.PlayerIDList`))
  ;[1 1 1] 通知全体玩家，更新界面
  (`KismetArrayLibrary.Array_Clear` (`self.TempGender`))
  (`KismetSystemLibrary.PrintString` (`KismetStringLibrary.Concat_StrStr` "更新【" (`KismetStringLibrary.Conv_IntToString` (`KismetArrayLibrary.Array_Length` _playeridlist)) "】个客户端"))
  (for _array_element _playeridlist
    (bind ((`Gender_9_04CBE3DF41AD94DD05ABAD8895DA80CA` _gender) (`PlayerController_14_0CFF2C2243D3BB09CA066A88EA0952CA` _playercontroller)) (break `/Game/Resource/BP/GameMode/GamePrepare_GameMode/BP_GamePrepare_PlayerInfor` _array_element))
    (bind _asbp_gp_player_ready (cast `/Game/Resource/BP/GameMode/GamePrepare_GameMode/BP_GP_PlayerReady` (`Controller.K2_GetPawn` _playercontroller)))
    (`KismetArrayLibrary.Array_Add` (`self.TempGender`) _gender)
    (`/Game/Resource/BP/GameMode/GamePrepare_GameMode/BP_GP_PlayerReady.Client_UpdateGameReadyWidget` _asbp_gp_player_ready _playercontroller _playeridlist))
  (`/Game/Resource/BP/GameMode/GamePrepare_GameMode/BP_GP_PC.Client_UpdateRoomInfor` (`.PlayerController_14_0CFF2C2243D3BB09CA066A88EA0952CA` (break `/Game/Resource/BP/GameMode/GamePrepare_GameMode/BP_GamePrepare_PlayerInfor` (`|GetArrayItem` (`self.PlayerIDList`)))) (`self.TempGender`)))

(event `Server_PlayerLogoutFromPlayerID`
  (params (PlayerID :type String))
  ;[1 1 1] 通过玩家ID让玩家退出游戏
  (for _array_element (`self.PlayerIDList`)
    (bind ((`PlayerController_14_0CFF2C2243D3BB09CA066A88EA0952CA` _playercontroller)) (break `/Game/Resource/BP/GameMode/GamePrepare_GameMode/BP_GamePrepare_PlayerInfor` _array_element))
    (if (`KismetStringLibrary.EqualEqual_StrStr` PlayerID (`/Game/Resource/BP/GameMode/GamePrepare_GameMode/BP_GP_PC.PlayerID` _playercontroller))
      (`/Game/Resource/BP/GameMode/GamePrepare_GameMode/BP_GP_PC.Client_Logout` _playercontroller)
      (break))))

(event `Server_GameStartAll`
  ;[1 1 1] 通知所有客户端，准备转移地图
  (for _array_element (`self.PlayerIDList`)
    (bind _asbp_gp_player_ready (cast `/Game/Resource/BP/GameMode/GamePrepare_GameMode/BP_GP_PlayerReady` (`Controller.K2_GetPawn` (`.PlayerController_14_0CFF2C2243D3BB09CA066A88EA0952CA` (break `/Game/Resource/BP/GameMode/GamePrepare_GameMode/BP_GamePrepare_PlayerInfor` _array_element)))))
    (`/Game/Resource/BP/GameMode/GamePrepare_GameMode/BP_GP_PlayerReady.Client_GameStart` _asbp_gp_player_ready)))

(event `Server_GameStart`
  ;[1 1 1] 开始游戏
  (bind _asbp_game_prepare_gs (cast `/Game/Resource/BP/GameMode/GamePrepare_GameMode/BP_GamePrepare_GS` (`GameplayStatics.GetGameState`)))
  (if (== (- (`KismetArrayLibrary.Array_Length` (`self.PlayerIDList`)) 1) (`KismetArrayLibrary.Array_Length` (`/Game/Resource/BP/GameMode/GamePrepare_GameMode/BP_GamePrepare_GS.ReadyID` _asbp_game_prepare_gs)))
    (`KismetSystemLibrary.PrintString` "开始，进入倒计时")
    (`self.Server_GameStartAll`)
    (else
      (`WidgetBase.CreateTipWidget` "还有玩家未准备"))))

(event `self.K2_PostLogin`
  (params (NewPlayer :type "PlayerController Object Reference"))
  ;[1 1 1] 玩家登录-准备界面-分配玩家ID号
  (bind _asbp_gp_pc (cast `/Game/Resource/BP/GameMode/GamePrepare_GameMode/BP_GP_PC` NewPlayer))
  (bind _output_get (set `self.NewLoginPlayerID` (`self.GetNow` _asbp_gp_pc)))
  (`self.Server_PlayerLogin` (make `/Game/Resource/BP/GameMode/GamePrepare_GameMode/BP_GamePrepare_PlayerInfor` :`PlayerController` _asbp_gp_pc :`PlayerID` _output_get)))

(event `self.K2_OnLogout`
  (params (ExitingController :type "Controller Object Reference"))
  ;[1 1 1] 角色离开-任何情况下的离开
  (`/Engine/EditorBlueprintResources/StandardMacros.IsValid` ExitingController
    (:`Is Valid`
      (bind _asbp_gp_pc (cast `/Game/Resource/BP/GameMode/GamePrepare_GameMode/BP_GP_PC` ExitingController))
      (`/Engine/EditorBlueprintResources/StandardMacros.IsValid` _asbp_gp_pc
        (:`Is Valid`
          (bind _bresult (`self.Remove Player Infor` (`/Game/Resource/BP/GameMode/GamePrepare_GameMode/BP_GP_PC.PlayerID` _asbp_gp_pc)))
          (if _bresult
            (`self.Server_UpdateAllPlayer`)))))))

(event `self.ReceiveBeginPlay`
  ;[1 1 1] 角色离开-任何情况下的离开
)

(fn `Check Player`
  (params (NewPlayer :type "/Game/Resource/BP/GameMode/GamePrepare_GameMode/BP_GamePrepare_PlayerInfor Structure"))
  (returns (PlayerInfor :type "/Game/Resource/BP/GameMode/GamePrepare_GameMode/BP_GamePrepare_PlayerInfor Structure") (Result :type Boolean))
  (bind _asbp_game_prepare_gs (cast `/Game/Resource/BP/GameMode/GamePrepare_GameMode/BP_GamePrepare_GS` (`GameplayStatics.GetGameState`))
    (:`then`
      (if (< (`KismetArrayLibrary.Array_Length` (`self.PlayerIDList`)) (`/Game/Resource/BP/GameMode/GamePrepare_GameMode/BP_GamePrepare_GS.PlayerNumMax` _asbp_game_prepare_gs))
        (return NewPlayer true)
        (else
          (return NewPlayer false))))
    (:`CastFailed`
      (`KismetSystemLibrary.PrintString` "游戏状态无效"))))

(fn `CheckHasPlayer`
  (params (PlayerID :type String))
  (returns (Result :type Boolean) (PlayerInfor :type "/Game/Resource/BP/GameMode/GamePrepare_GameMode/BP_GamePrepare_PlayerInfor Structure"))
  (for _array_element (`self.PlayerIDList`)
    (if (`KismetStringLibrary.EqualEqual_StrStr` (`.PlayerID_17_82A6292246D93206D86F94827F3246E7` (break `/Game/Resource/BP/GameMode/GamePrepare_GameMode/BP_GamePrepare_PlayerInfor` _array_element)) (`local.PlayerID`))
      (return true _array_element)))
  (return false))

(fn `GetNow`
  (params (PlayerCtrl :type "PlayerController Object Reference"))
  (returns (TimeStr :type String))
  (bind (_returnvalue_year _returnvalue_month _returnvalue_day _returnvalue_hour _returnvalue_minute _returnvalue_second _returnvalue_millisecond) (`KismetMathLibrary.BreakDateTime` (`KismetMathLibrary.Now`)))
  (return (`KismetStringLibrary.Concat_StrStr` (`KismetStringLibrary.Conv_IntToString` _returnvalue_year) (`KismetStringLibrary.Conv_IntToString` _returnvalue_month) (`KismetStringLibrary.Conv_IntToString` _returnvalue_day) (`KismetStringLibrary.Conv_IntToString` _returnvalue_hour) (`KismetStringLibrary.Conv_IntToString` _returnvalue_minute) (`KismetStringLibrary.Conv_IntToString` _returnvalue_second) (`KismetStringLibrary.Conv_IntToString` _returnvalue_millisecond) (`KismetSystemLibrary.GetObjectName` PlayerCtrl))))

(fn `GetPlayerList`
  (returns (PlayerIDList :type "Array of /Game/Resource/BP/GameMode/GamePrepare_GameMode/BP_GamePrepare_PlayerInfor Structure"))
  (return (`self.PlayerIDList`)))

(fn `JoinFailed`
  (params (PlayerInfor :type "/Game/Resource/BP/GameMode/GamePrepare_GameMode/BP_GamePrepare_PlayerInfor Structure"))
  (bind ((`PlayerController_14_0CFF2C2243D3BB09CA066A88EA0952CA` _playercontroller)) (break `/Game/Resource/BP/GameMode/GamePrepare_GameMode/BP_GamePrepare_PlayerInfor` PlayerInfor))
  (`/Engine/EditorBlueprintResources/StandardMacros.IsValid` _playercontroller
    (:`Is Valid`
      (`/Game/Resource/BP/GameMode/GamePrepare_GameMode/BP_GP_PC.Client_Logout` _playercontroller))))

(fn `MoveTempPlayerInfor`
  (params (MoveValue :type "/Game/Resource/BP/GameMode/GamePrepare_GameMode/BP_GamePrepare_PlayerInfor Structure"))
  (returns (Result :type Boolean))
  (locals (NewPlayerInfor :type "/Game/Resource/BP/GameMode/GamePrepare_GameMode/BP_GamePrepare_PlayerInfor Structure"))
  (set `local.NewPlayerInfor` MoveValue)
  (for (_array_element _array_index) (`self.TempList`)
    (bind ((`PlayerController_14_0CFF2C2243D3BB09CA066A88EA0952CA` _playercontroller) (`PlayerID_17_82A6292246D93206D86F94827F3246E7` _playerid)) (break `/Game/Resource/BP/GameMode/GamePrepare_GameMode/BP_GamePrepare_PlayerInfor` _array_element))
    (if (`KismetStringLibrary.EqualEqual_StrStr` (`.PlayerID_17_82A6292246D93206D86F94827F3246E7` (break `/Game/Resource/BP/GameMode/GamePrepare_GameMode/BP_GamePrepare_PlayerInfor` (`local.NewPlayerInfor`))) _playerid)
      (bind _structout (setmembers `/Game/Resource/BP/GameMode/GamePrepare_GameMode/BP_GamePrepare_PlayerInfor` :`StructRef` (`local.NewPlayerInfor`) :`PlayerController` _playercontroller))
      (`KismetArrayLibrary.Array_Add` (`self.PlayerIDList`) _structout)
      (`KismetArrayLibrary.Array_Remove` (`self.TempList`) _array_index)
      (return true)))
  (return false))

(fn `Remove Player Infor`
  (params (PlayerID :type String))
  (returns (bResult :type Boolean))
  (locals (GS :type "/Game/Resource/BP/GameMode/GamePrepare_GameMode/BP_GamePrepare_GS Object Reference"))
  (bind _asbp_game_prepare_gs (cast `/Game/Resource/BP/GameMode/GamePrepare_GameMode/BP_GamePrepare_GS` (`GameplayStatics.GetGameState`)))
  (set `local.GS` _asbp_game_prepare_gs)
  (if (`KismetStringLibrary.EqualEqual_StrStr` (`local.PlayerID`) (`/Game/Resource/BP/GameMode/GamePrepare_GameMode/BP_GamePrepare_GS.RoomOwnerID` (`local.GS`)))
    (return false)
    (else
      (if (`KismetArrayLibrary.Array_Contains` (`/Game/Resource/BP/GameMode/GamePrepare_GameMode/BP_GamePrepare_GS.ReadyID` (`local.GS`)) (`local.PlayerID`))
        (`KismetArrayLibrary.Array_RemoveItem` (`/Game/Resource/BP/GameMode/GamePrepare_GameMode/BP_GamePrepare_GS.ReadyID` (`local.GS`)) (`local.PlayerID`)))
      (for (_array_element _array_index) (`self.PlayerIDList`)
        (if (`KismetStringLibrary.EqualEqual_StrStr` (`local.PlayerID`) (`.PlayerID_17_82A6292246D93206D86F94827F3246E7` (break `/Game/Resource/BP/GameMode/GamePrepare_GameMode/BP_GamePrepare_PlayerInfor` _array_element)))
          (`KismetArrayLibrary.Array_Remove` (`self.PlayerIDList`) _array_index)
          (return true)))
      (return false))))

(fn `UserConstructionScript`)